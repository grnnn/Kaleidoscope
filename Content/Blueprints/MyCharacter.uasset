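; Player character Blueprint that provides a pause menu and holds several fixed-angle camera spring arms.
; BeginPlay creates the menu widget, and P or Escape toggles it along with game pause, input mode and cursor.
; Tick re-pins the spring arms' world rotations, plus two of their relative locations.
; A Trace function highlights looked-at static meshes via custom depth, but its timer, like the camera-rotation logic, is disconnected.
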(event EventBeginPlay
  ;[1 1 1] Game Pause Menu
  (bind _returnvalue (UserInterface|CreateWidget "/Game/Blueprints/z-mainMenu/0-PauseMenu.0-PauseMenu_C" (Game|GetPlayerController 0)))
  (Variables|Default|SetMyMenu _returnvalue))

(event EventTick
  (params (DeltaSeconds :type Float%20%28single-precision%29))
  (bind _springarm3_sideview (Variables|Default|GetSpringArm3_sideview))
  (bind _springarm3_right_hand_side (Variables|Default|GetSpringArm3_right_hand_side))
  (Transformation|SetWorldRotation _springarm3_right_hand_side "0,390.000000, 0" false)
  (Transformation|SetRelativeLocation _springarm3_right_hand_side "0, 0,60.000000" false)
  (Transformation|SetWorldRotation _springarm3_sideview "0.000000,130.000000,0.000000" false)
  (Transformation|SetRelativeLocation _springarm3_sideview "0.000000,0.000000,60.000000" false)
  (Transformation|SetWorldRotation (Variables|Default|GetSpringArm2_roadside) "0,30.000000, 0" false)
  (Transformation|SetWorldRotation (Variables|Default|GetSpringArm_roadsize_close_look) "0.000000,260.000000, 0" false)
  (Transformation|SetWorldRotation (Variables|Default|GetSpringArm_s6_side) "-5.000000,-90.000000, 0" false)
  (Transformation|SetWorldRotation (Variables|Default|GetSpringArm_s6_second) "0,-144.999969, 0" false))

(event Input|KeyboardEvents|P
  (bind _returnvalue (Game|GetPlayerController 0))
  (bind _mymenu (Variables|Default|GetMyMenu))
  ;[1 1 1] Game Pause Menu
  (:Released
    (if (Variables|Default|GetpauseOn)
      (Widget|RemovefromParent _mymenu)
      (Input|SetInputModeGameOnly _returnvalue)
      (Variables|/Script/Engine.PlayerController|SetbShowMouseCursor _returnvalue false)
      (Game|SetGamePaused 0 false)
      (Variables|Default|SetpauseOn false)
      (else
        (UserInterface|Viewport|AddtoViewport _mymenu)
        (Input|SetInputModeGameandUI _returnvalue _mymenu false true)
        (Variables|/Script/Engine.PlayerController|SetbShowMouseCursor _returnvalue true)
        (Game|SetGamePaused 0 true)
        (Variables|Default|SetpauseOn true)))))

(event Input|KeyboardEvents|Escape
  (bind _returnvalue (Game|GetPlayerController 0))
  (bind _mymenu (Variables|Default|GetMyMenu))
  ;[1 1 1] Game Pause Menu
  (:Released
    (if (Variables|Default|GetpauseOn)
      (Widget|RemovefromParent _mymenu)
      (Input|SetInputModeGameOnly _returnvalue)
      (Variables|/Script/Engine.PlayerController|SetbShowMouseCursor _returnvalue false)
      (Game|SetGamePaused 0 false)
      (Variables|Default|SetpauseOn false)
      (else
        (UserInterface|Viewport|AddtoViewport _mymenu)
        (Input|SetInputModeGameandUI _returnvalue _mymenu false true)
        (Variables|/Script/Engine.PlayerController|SetbShowMouseCursor _returnvalue true)
        (Game|SetGamePaused 0 true)
        (Variables|Default|SetpauseOn true)))))

(fn ConstructionScript)

(fn Trace
  (bind _followcamera (Variables|Default|GetFollowCamera))
  (bind _returnvalue (Transformation|GetWorldLocation _followcamera))
  ;[1 1 1] Get where the character is looking at, then highlight any mesh object within the view
  (bind (_outhit _returnvalue_2) (Collision|LineTraceByChannel 0 _returnvalue (+ _returnvalue (* (Math|Vector|GetForwardVector (.Rotation (Math|Transform|BreakTransform (Transformation|GetWorldTransform (Variables|Default|GetFollowCamera))))) 5e+02)) "TraceTypeQuery1" false 0 "None"))
  (if _returnvalue_2
    (bind _asstatic_mesh_component (Utilities|Casting|CastToStaticMeshComponent (.HitComponent (Collision|BreakHitResult _outhit)))
      (:then
        (if (== (Variables|Default|GetCurrent%20Target) _asstatic_mesh_component)
          _
          (else
            (Rendering|SetRenderCustomDepth (Variables|Default|GetCurrent%20Target) false)))
        (Variables|Default|SetCurrent%20Target _asstatic_mesh_component)
        (Rendering|SetRenderCustomDepth _asstatic_mesh_component true))
      (:CastFailed
        (Utilities|IsValid (Variables|Default|GetCurrent%20Target) :!label _label
          (:Is%20Valid
            (Rendering|SetRenderCustomDepth (Variables|Default|GetCurrent%20Target) false)
            (Variables|Default|SetCurrent%20Target 0)))))
    (else
      (goto _label))))