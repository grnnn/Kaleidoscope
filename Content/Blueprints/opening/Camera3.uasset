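; Camera3 is an opening camera actor that follows the player's MyCharacter.
; Every tick it copies the transform of the character's FollowCamera, shifted by a fixed world-space offset along negative X and downward in Z, keeping rotation and scale.
; An attach to the SpringArmOpening component and a debug location print are left disconnected and never run.
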(event EventTick
  (params (DeltaSeconds :type Float%20%28single-precision%29))
  ;[1 1 1] Make this camera to follow the main character
  (bind _asmy_character (Utilities|Casting|CastToMyCharacter (Game|GetPlayerCharacter 0)))
  (Transformation|SetWorldTransform (Math|Transform|MakeTransform (Math|Vector|MakeVector (+ (.X (Math|Vector|BreakVector (.Location (Math|Transform|BreakTransform (Transformation|GetWorldTransform (Variables|/Script/Kaleidoscope.KaleidoscopeCharacter|GetFollowCamera _asmy_character)))))) -2e+02) (.Y (Math|Vector|BreakVector (.Location (Math|Transform|BreakTransform (Transformation|GetWorldTransform (Variables|/Script/Kaleidoscope.KaleidoscopeCharacter|GetFollowCamera _asmy_character)))))) (+ (.Z (Math|Vector|BreakVector (.Location (Math|Transform|BreakTransform (Transformation|GetWorldTransform (Variables|/Script/Kaleidoscope.KaleidoscopeCharacter|GetFollowCamera _asmy_character)))))) -1e+02)) (.Rotation (Math|Transform|BreakTransform (Transformation|GetWorldTransform (Variables|/Script/Kaleidoscope.KaleidoscopeCharacter|GetFollowCamera _asmy_character)))) (.Scale (Math|Transform|BreakTransform (Transformation|GetWorldTransform (Variables|/Script/Kaleidoscope.KaleidoscopeCharacter|GetFollowCamera _asmy_character))))) false))

(fn ConstructionScript)