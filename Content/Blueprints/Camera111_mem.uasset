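; Camera actor that slowly pans its Camera1 component once Triggered is set, which the author's note ties to the player triggering a sign.
; Each Tick first counts HoldSec down as a delay, then steps the yaw slightly negative until Counter reaches zero, so timing depends on frame rate.
; A disconnected sphere-trace branch for detecting KaleidoscopeCharacter in front of the camera is left unused.
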(event EventTick
  (params (DeltaSeconds :type Float%20%28single-precision%29))
  (bind _camera1 (Variables|Default|GetCamera1))
  (bind _returnvalue (Transformation|GetWorldRotation _camera1))
  (bind (_pitch _yaw _roll) (Class|KismetMathLibrary|BreakRot _returnvalue))
  ;[1 1 1] When the player triggers the sign, camera rotates
  (if (Variables|Default|Gettriggered)
    (if (== (Variables|Default|Gethold_sec) 0)
      (if (not (== (Variables|Default|Getcounter) 0))
        (Transformation|SetWorldRotation _camera1 (Class|KismetMathLibrary|MakeRot _pitch (+ _yaw -0.1) _roll) false)
        (Variables|Default|Setcounter (- (Variables|Default|Getcounter) 1)))
      (else
        (Variables|Default|Sethold_sec (- (Variables|Default|Gethold_sec) 1))))))

(fn ConstructionScript)