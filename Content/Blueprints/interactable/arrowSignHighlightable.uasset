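; Interactable arrow sign that highlights while something overlaps its HighlightBox.
; The construction script creates dynamic material instances for the two material slots of the ArrowSign component, stored as DynamicPost and DynamicBoard.
; Begin overlap sets their "post" and "board" color parameters to white, and end overlap sets them back to hard-coded brown shades, with no filter on the overlapping actor.
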(event OnComponentBeginOverlap(HighlightBox)
  (params (OtherActor :type Actor%20Object%20Reference) (OtherComp :type Primitive%20Component%20Object%20Reference) (OtherBodyIndex :type Integer) (bFromSweep :type Boolean) (SweepResult :type Hit%20Result%20Structure%20%28by%20ref%29))
  ;[1 1 1] set highlight color
  (Utilities|FlowControl|Sequence
    (:then_0
      (Rendering|Material|SetVectorParameterValue (Variables|Default|GetDynamicPost) "post" "(R=1.000000,G=1.000000,B=1.000000,A=1.000000)" :!class /Script/Engine.MaterialInstanceDynamic))
    (:then_1
      (Rendering|Material|SetVectorParameterValue (Variables|Default|GetDynamicBoard) "board" "(R=1.000000,G=1.000000,B=1.000000,A=1.000000)" :!class /Script/Engine.MaterialInstanceDynamic))))

(event OnComponentEndOverlap(HighlightBox)
  (params (OtherActor :type Actor%20Object%20Reference) (OtherComp :type Primitive%20Component%20Object%20Reference) (OtherBodyIndex :type Integer))
  ;[1 1 1] set back to proper color
  (Utilities|FlowControl|Sequence
    (:then_0
      (Rendering|Material|SetVectorParameterValue (Variables|Default|GetDynamicPost) "post" "(R=0.084000,G=0.037000,B=0.017000,A=1.000000)" :!class /Script/Engine.MaterialInstanceDynamic))
    (:then_1
      (Rendering|Material|SetVectorParameterValue (Variables|Default|GetDynamicBoard) "board" "(R=0.179000,G=0.097000,B=0.057000,A=1.000000)" :!class /Script/Engine.MaterialInstanceDynamic))))

(fn ConstructionScript
  (bind _arrowsign (Variables|Default|GetarrowSign))
  (Utilities|FlowControl|Sequence
    (:then_0
      (bind _returnvalue (Rendering|Material|CreateDynamicMaterialInstance _arrowsign 0 0 :!class /Script/Engine.PrimitiveComponent))
      (Variables|Default|SetDynamicPost _returnvalue))
    (:then_1
      (bind _returnvalue_2 (Rendering|Material|CreateDynamicMaterialInstance _arrowsign 1 0 :!class /Script/Engine.PrimitiveComponent))
      (Variables|Default|SetDynamicBoard _returnvalue_2))))