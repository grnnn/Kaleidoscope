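; Interactable coffee table that highlights when something overlaps its HighlightBox trigger.
; The construction script creates a dynamic material instance on the CoffeeTable's first material slot, stored as DynamicPost.
; Overlap begin sets that instance's "wood" color parameter to near-white, and overlap end sets it back to a hardcoded brown.
; A FirstTime check follows the highlight but leads to no action.
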(event OnComponentBeginOverlap(highlightBox)
  (params (OtherActor :type Actor%20Object%20Reference) (OtherComp :type Primitive%20Component%20Object%20Reference) (OtherBodyIndex :type Integer) (bFromSweep :type Boolean) (SweepResult :type Hit%20Result%20Structure%20%28by%20ref%29))
  ;[1 1 1] set to highlight color
  (Rendering|Material|SetVectorParameterValue (Variables|Default|GetDynamicPost) "wood" "(R=0.989000,G=0.989000,B=0.989000,A=1.000000)" :!class /Script/Engine.MaterialInstanceDynamic)
  (if (Variables|Default|GetFirstTime)
    _))

(event OnComponentEndOverlap(highlightBox)
  (params (OtherActor :type Actor%20Object%20Reference) (OtherComp :type Primitive%20Component%20Object%20Reference) (OtherBodyIndex :type Integer))
  ;[1 1 1] set back to proper color
  (Rendering|Material|SetVectorParameterValue (Variables|Default|GetDynamicPost) "wood" "(R=0.335000,G=0.257000,B=0.201000,A=1.000000)" :!class /Script/Engine.MaterialInstanceDynamic))

(fn ConstructionScript
  (bind _returnvalue (Rendering|Material|CreateDynamicMaterialInstance (Variables|Default|GetcoffeeTable) 0 0 :!class /Script/Engine.PrimitiveComponent))
  (Variables|Default|SetDynamicPost _returnvalue))