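; Interactable basket that highlights by turning near-white while something overlaps its HighlightBox, then returns to its wood colors when the overlap ends.
; The construction script creates dynamic material instances for the light, dark and handle slots, and overlap events set their "wood" vector parameter.
; Tick polls a Check flag and, when true, calls DestroyComponent and reuses the end-overlap path to restore the original colors.
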(event OnComponentBeginOverlap(highlightBox)
  (params (OtherActor :type Actor%20Object%20Reference) (OtherComp :type Primitive%20Component%20Object%20Reference) (OtherBodyIndex :type Integer) (bFromSweep :type Boolean) (SweepResult :type Hit%20Result%20Structure%20%28by%20ref%29))
  ;[1 1 1] set to highlight color
  (Utilities|FlowControl|Sequence
    (:then_0
      (Rendering|Material|SetVectorParameterValue (Variables|Default|GetDynamicLight) "wood" "(R=0.989000,G=0.989000,B=0.989000,A=1.000000)" :!class /Script/Engine.MaterialInstanceDynamic))
    (:then_1
      (Rendering|Material|SetVectorParameterValue (Variables|Default|GetDynamicDark) "wood" "(R=1.000000,G=1.000000,B=1.000000,A=1.000000)" :!class /Script/Engine.MaterialInstanceDynamic))
    (:then_2
      (Rendering|Material|SetVectorParameterValue (Variables|Default|GetDynamicHandle) "wood" "(R=1.000000,G=1.000000,B=1.000000,A=1.000000)" :!class /Script/Engine.MaterialInstanceDynamic))))

(event OnComponentEndOverlap(highlightBox)
  (params (OtherActor :type Actor%20Object%20Reference) (OtherComp :type Primitive%20Component%20Object%20Reference) (OtherBodyIndex :type Integer))
  ;[1 1 1] set back to proper color
  (Utilities|FlowControl|Sequence
    (:then_0
      (Rendering|Material|SetVectorParameterValue (Variables|Default|GetDynamicLight) "wood" "(R=0.758000,G=0.403000,B=0.151000,A=1.000000)" :!class /Script/Engine.MaterialInstanceDynamic))
    (:then_1
      (Rendering|Material|SetVectorParameterValue (Variables|Default|GetDynamicDark) "wood" "(R=0.674000,G=0.359000,B=0.135000,A=1.000000)" :!class /Script/Engine.MaterialInstanceDynamic))
    (:then_2
      (Rendering|Material|SetVectorParameterValue (Variables|Default|GetDynamicHandle) "wood" "(R=0.137000,G=0.013300,B=0.000000,A=1.000000)" :!class /Script/Engine.MaterialInstanceDynamic))))

(event EventTick
  (params (DeltaSeconds :type Float%20%28single-precision%29))
  (if (Variables|Default|Getcheck)
    (Components|DestroyComponent)
    ;[1 1 1] set back to proper color
    (Utilities|FlowControl|Sequence
      (:then_0
        (Rendering|Material|SetVectorParameterValue (Variables|Default|GetDynamicLight) "wood" "(R=0.758000,G=0.403000,B=0.151000,A=1.000000)" :!class /Script/Engine.MaterialInstanceDynamic))
      (:then_1
        (Rendering|Material|SetVectorParameterValue (Variables|Default|GetDynamicDark) "wood" "(R=0.674000,G=0.359000,B=0.135000,A=1.000000)" :!class /Script/Engine.MaterialInstanceDynamic))
      (:then_2
        (Rendering|Material|SetVectorParameterValue (Variables|Default|GetDynamicHandle) "wood" "(R=0.137000,G=0.013300,B=0.000000,A=1.000000)" :!class /Script/Engine.MaterialInstanceDynamic)))))

(fn ConstructionScript
  (bind _basket (Variables|Default|Getbasket))
  (Utilities|FlowControl|Sequence
    (:then_0
      (bind _returnvalue (Rendering|Material|CreateDynamicMaterialInstance _basket 0 0 :!class /Script/Engine.PrimitiveComponent))
      (Variables|Default|SetDynamicLight _returnvalue))
    (:then_1
      (bind _returnvalue_2 (Rendering|Material|CreateDynamicMaterialInstance _basket 1 0 :!class /Script/Engine.PrimitiveComponent))
      (Variables|Default|SetDynamicDark _returnvalue_2))
    (:then_2
      (bind _returnvalue_3 (Rendering|Material|CreateDynamicMaterialInstance _basket 2 0 :!class /Script/Engine.PrimitiveComponent))
      (Variables|Default|SetDynamicHandle _returnvalue_3))))