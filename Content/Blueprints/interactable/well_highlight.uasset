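; Well highlight interactable that tints its material while something overlaps its Box1 trigger.
; The construction script creates a dynamic material instance, whose "base" color turns white on begin overlap and returns to dark brown on end overlap.
; Once the Check flag is true, begin overlap no longer highlights, and Tick calls DestroyComponent and restores the brown color, with no guard against repeating each frame.
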(event OnComponentBeginOverlap(Box1)
  (params (OtherActor :type Actor%20Object%20Reference) (OtherComp :type Primitive%20Component%20Object%20Reference) (OtherBodyIndex :type Integer) (bFromSweep :type Boolean) (SweepResult :type Hit%20Result%20Structure%20%28by%20ref%29))
  (if (not (Variables|Default|Getcheck))
    (Rendering|Material|SetVectorParameterValue (Variables|Default|GetNewVar) "base" "(R=1.000000,G=1.000000,B=1.000000,A=1.000000)" :!class /Script/Engine.MaterialInstanceDynamic)))

(event OnComponentEndOverlap(Box1)
  (params (OtherActor :type Actor%20Object%20Reference) (OtherComp :type Primitive%20Component%20Object%20Reference) (OtherBodyIndex :type Integer))
  (Rendering|Material|SetVectorParameterValue (Variables|Default|GetNewVar) "base" "(R=0.054902,G=0.031373,B=0.015686,A=0.000000)" :!class /Script/Engine.MaterialInstanceDynamic))

(event EventTick
  (params (DeltaSeconds :type Float%20%28single-precision%29))
  (if (Variables|Default|Getcheck)
    (Components|DestroyComponent)
    (Rendering|Material|SetVectorParameterValue (Variables|Default|GetNewVar) "base" "(R=0.054902,G=0.031373,B=0.015686,A=0.000000)" :!class /Script/Engine.MaterialInstanceDynamic)))

(fn ConstructionScript
  (bind _returnvalue (Rendering|Material|CreateDynamicMaterialInstance 0 0 :!class /Script/Engine.PrimitiveComponent))
  (Variables|Default|SetNewVar _returnvalue))