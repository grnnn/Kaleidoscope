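; Interactable teacher desk highlight that changes the desk's material color while something overlaps its trigger box.
; The construction script creates a dynamic material instance on the first material slot, and the box's begin and end overlap events switch its Base color between near-white and dark brown.
; Tick polls a Check flag and, when true, destroys a component and restores the dark color.
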(event OnComponentEndOverlap(Box1)
  (params (OtherActor :type Actor%20Object%20Reference) (OtherComp :type Primitive%20Component%20Object%20Reference) (OtherBodyIndex :type Integer))
  (Rendering|Material|SetVectorParameterValue (Variables|Default|GetNewVar) "Base" "(R=0.074510,G=0.023529,B=0.007843,A=0.000000)" :!class /Script/Engine.MaterialInstanceDynamic))

(event OnComponentBeginOverlap(Box1)
  (params (OtherActor :type Actor%20Object%20Reference) (OtherComp :type Primitive%20Component%20Object%20Reference) (OtherBodyIndex :type Integer) (bFromSweep :type Boolean) (SweepResult :type Hit%20Result%20Structure%20%28by%20ref%29))
  (Rendering|Material|SetVectorParameterValue (Variables|Default|GetNewVar) "Base" "(R=0.992157,G=0.992157,B=0.992157,A=1.000000)" :!class /Script/Engine.MaterialInstanceDynamic))

(event EventTick
  (params (DeltaSeconds :type Float%20%28single-precision%29))
  (if (Variables|Default|Getcheck)
    (Components|DestroyComponent)
    (Rendering|Material|SetVectorParameterValue (Variables|Default|GetNewVar) "Base" "(R=0.074510,G=0.023529,B=0.007843,A=0.000000)" :!class /Script/Engine.MaterialInstanceDynamic)))

(fn ConstructionScript
  (bind _returnvalue (Rendering|Material|CreateDynamicMaterialInstance 0 0 :!class /Script/Engine.PrimitiveComponent))
  (Variables|Default|SetNewVar _returnvalue))