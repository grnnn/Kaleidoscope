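; Interactable luggage prop that highlights while something overlaps its HighlightBox.
; The construction script creates dynamic material instances for the Luggage mesh's base, strap, button and top slots.
; Begin overlap sets their "wood" or "brass" color parameters to near white, and end overlap restores hardcoded original colors.
; Overlaps are not filtered by actor or counted, so any exit clears the highlight.
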(event OnComponentBeginOverlap(highlightBox)
  (params (OtherActor :type Actor%20Object%20Reference) (OtherComp :type Primitive%20Component%20Object%20Reference) (OtherBodyIndex :type Integer) (bFromSweep :type Boolean) (SweepResult :type Hit%20Result%20Structure%20%28by%20ref%29))
  ;[1 1 1] set to highlight color
  (Utilities|FlowControl|Sequence
    (:then_0
      (Rendering|Material|SetVectorParameterValue (Variables|Default|GetDynamicBase) "wood" "(R=0.989000,G=0.989000,B=0.989000,A=1.000000)" :!class /Script/Engine.MaterialInstanceDynamic))
    (:then_1
      (Rendering|Material|SetVectorParameterValue (Variables|Default|GetDynamicStrap) "wood" "(R=1.000000,G=1.000000,B=1.000000,A=1.000000)" :!class /Script/Engine.MaterialInstanceDynamic))
    (:then_2
      (Rendering|Material|SetVectorParameterValue (Variables|Default|GetDynamicButton) "brass" "(R=1.000000,G=1.000000,B=1.000000,A=1.000000)" :!class /Script/Engine.MaterialInstanceDynamic))
    (:then_3
      (Rendering|Material|SetVectorParameterValue (Variables|Default|GetDynamicTop) "wood" "(R=1.000000,G=1.000000,B=1.000000,A=1.000000)" :!class /Script/Engine.MaterialInstanceDynamic))))

(event OnComponentEndOverlap(highlightBox)
  (params (OtherActor :type Actor%20Object%20Reference) (OtherComp :type Primitive%20Component%20Object%20Reference) (OtherBodyIndex :type Integer))
  ;[1 1 1] set back to proper color
  (Utilities|FlowControl|Sequence
    (:then_0
      (Rendering|Material|SetVectorParameterValue (Variables|Default|GetDynamicBase) "wood" "(R=0.101961,G=0.031373,B=0.011765,A=0.000000)" :!class /Script/Engine.MaterialInstanceDynamic))
    (:then_1
      (Rendering|Material|SetVectorParameterValue (Variables|Default|GetDynamicStrap) "wood" "(R=0.058824,G=0.023529,B=0.007843,A=0.000000)" :!class /Script/Engine.MaterialInstanceDynamic))
    (:then_2
      (Rendering|Material|SetVectorParameterValue (Variables|Default|GetDynamicButton) "brass" "(R=0.368627,G=0.243137,B=0.050980,A=0.000000)" :!class /Script/Engine.MaterialInstanceDynamic))
    (:then_3
      (Rendering|Material|SetVectorParameterValue (Variables|Default|GetDynamicTop) "wood" "(R=0.141176,G=0.035294,B=0.007843,A=0.000000)" :!class /Script/Engine.MaterialInstanceDynamic))))

(fn ConstructionScript
  (bind _luggage (Variables|Default|Getluggage))
  (Utilities|FlowControl|Sequence
    (:then_0
      (bind _returnvalue (Rendering|Material|CreateDynamicMaterialInstance _luggage 0 0 :!class /Script/Engine.PrimitiveComponent))
      (Variables|Default|SetDynamicBase _returnvalue))
    (:then_1
      (bind _returnvalue_2 (Rendering|Material|CreateDynamicMaterialInstance _luggage 1 0 :!class /Script/Engine.PrimitiveComponent))
      (Variables|Default|SetDynamicStrap _returnvalue_2))
    (:then_2
      (bind _returnvalue_3 (Rendering|Material|CreateDynamicMaterialInstance _luggage 2 0 :!class /Script/Engine.PrimitiveComponent))
      (Variables|Default|SetDynamicButton _returnvalue_3))
    (:then_3
      (bind _returnvalue_4 (Rendering|Material|CreateDynamicMaterialInstance _luggage 3 0 :!class /Script/Engine.PrimitiveComponent))
      (Variables|Default|SetDynamicTop _returnvalue_4))))