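; Interactable board prop that highlights near-white while something overlaps its HighlightBox and returns to its green, brown and tan colors afterward.
; The construction script creates dynamic material instances for the top, frame and main slots of the Luggage mesh.
; Overlap events set each instance's color parameter.
; Tick polls the Check flag, which is not set here, and when true destroys a component and restores the normal colors.
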(event OnComponentBeginOverlap(highlightBox)
  (params (OtherActor :type Actor%20Object%20Reference) (OtherComp :type Primitive%20Component%20Object%20Reference) (OtherBodyIndex :type Integer) (bFromSweep :type Boolean) (SweepResult :type Hit%20Result%20Structure%20%28by%20ref%29))
  ;[1 1 1] set to highlight color
  (Utilities|FlowControl|Sequence
    (:then_0
      (Rendering|Material|SetVectorParameterValue (Variables|Default|GetDynamicTop) "green" "(R=0.989000,G=0.989000,B=0.989000,A=1.000000)" :!class /Script/Engine.MaterialInstanceDynamic))
    (:then_1
      (Rendering|Material|SetVectorParameterValue (Variables|Default|GetDynamicFrame) "brown" "(R=1.000000,G=1.000000,B=1.000000,A=1.000000)" :!class /Script/Engine.MaterialInstanceDynamic))
    (:then_2
      (Rendering|Material|SetVectorParameterValue (Variables|Default|GetDynamicMain) "tan" "(R=1.000000,G=1.000000,B=1.000000,A=1.000000)" :!class /Script/Engine.MaterialInstanceDynamic))))

(event OnComponentEndOverlap(highlightBox)
  (params (OtherActor :type Actor%20Object%20Reference) (OtherComp :type Primitive%20Component%20Object%20Reference) (OtherBodyIndex :type Integer))
  ;[1 1 1] set back to proper color
  (Utilities|FlowControl|Sequence
    (:then_0
      (Rendering|Material|SetVectorParameterValue (Variables|Default|GetDynamicTop) "green" "(R=0.298039,G=0.349020,B=0.164706,A=0.000000)" :!class /Script/Engine.MaterialInstanceDynamic))
    (:then_1
      (Rendering|Material|SetVectorParameterValue (Variables|Default|GetDynamicFrame) "brown" "(R=0.168627,G=0.074510,B=0.027451,A=0.000000)" :!class /Script/Engine.MaterialInstanceDynamic))
    (:then_2
      (Rendering|Material|SetVectorParameterValue (Variables|Default|GetDynamicMain) "tan" "(R=0.278431,G=0.149020,B=0.066667,A=0.000000)" :!class /Script/Engine.MaterialInstanceDynamic))))

(event EventTick
  (params (DeltaSeconds :type Float%20%28single-precision%29))
  (if (Variables|Default|Getcheck)
    (Components|DestroyComponent)
    ;[1 1 1] set back to proper color
    (Utilities|FlowControl|Sequence
      (:then_0
        (Rendering|Material|SetVectorParameterValue (Variables|Default|GetDynamicTop) "green" "(R=0.298039,G=0.349020,B=0.164706,A=0.000000)" :!class /Script/Engine.MaterialInstanceDynamic))
      (:then_1
        (Rendering|Material|SetVectorParameterValue (Variables|Default|GetDynamicFrame) "brown" "(R=0.168627,G=0.074510,B=0.027451,A=0.000000)" :!class /Script/Engine.MaterialInstanceDynamic))
      (:then_2
        (Rendering|Material|SetVectorParameterValue (Variables|Default|GetDynamicMain) "tan" "(R=0.278431,G=0.149020,B=0.066667,A=0.000000)" :!class /Script/Engine.MaterialInstanceDynamic)))))

(fn ConstructionScript
  (bind _luggage (Variables|Default|Getluggage))
  (Utilities|FlowControl|Sequence
    (:then_0
      (bind _returnvalue (Rendering|Material|CreateDynamicMaterialInstance _luggage 0 0 :!class /Script/Engine.PrimitiveComponent))
      (Variables|Default|SetDynamicTop _returnvalue))
    (:then_1
      (bind _returnvalue_2 (Rendering|Material|CreateDynamicMaterialInstance _luggage 1 0 :!class /Script/Engine.PrimitiveComponent))
      (Variables|Default|SetDynamicFrame _returnvalue_2))
    (:then_2
      (bind _returnvalue_3 (Rendering|Material|CreateDynamicMaterialInstance _luggage 2 0 :!class /Script/Engine.PrimitiveComponent))
      (Variables|Default|SetDynamicMain _returnvalue_3))))