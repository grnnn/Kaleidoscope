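; Interactable board Blueprint that highlights itself while something overlaps its highlight box.
; The construction script creates a dynamic material instance on the Board component's first material slot.
; Begin and end overlap events on HighlightBox switch that instance's "wood" vector parameter between white and a hard-coded brown, with no filtering on the overlapping actor.
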(event OnComponentBeginOverlap(HighlightBox)
  (params (OtherActor :type Actor%20Object%20Reference) (OtherComp :type Primitive%20Component%20Object%20Reference) (OtherBodyIndex :type Integer) (bFromSweep :type Boolean) (SweepResult :type Hit%20Result%20Structure%20%28by%20ref%29))
  ;[1 1 1] set highlight color
  (Utilities|FlowControl|Sequence
    (:then_0
      (Rendering|Material|SetVectorParameterValue (Variables|Default|GetDynamicBoard) "wood" "(R=1.000000,G=1.000000,B=1.000000,A=1.000000)" :!class /Script/Engine.MaterialInstanceDynamic))))

(event OnComponentEndOverlap(HighlightBox)
  (params (OtherActor :type Actor%20Object%20Reference) (OtherComp :type Primitive%20Component%20Object%20Reference) (OtherBodyIndex :type Integer))
  ;[1 1 1] set back to proper color
  (Utilities|FlowControl|Sequence
    (:then_0
      (Rendering|Material|SetVectorParameterValue (Variables|Default|GetDynamicBoard) "wood" "(R=0.253000,G=0.181000,B=0.112000,A=1.000000)" :!class /Script/Engine.MaterialInstanceDynamic))))

(fn ConstructionScript
  (Utilities|FlowControl|Sequence
    (:then_0
      (bind _returnvalue (Rendering|Material|CreateDynamicMaterialInstance (Variables|Default|Getboard) 0 0 :!class /Script/Engine.PrimitiveComponent))
      (Variables|Default|SetDynamicBoard _returnvalue))))