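; Interactable opening sign that lights up near-white while something overlaps its HighlightBox.
; The construction script creates dynamic material instances for the sign mesh's three slots: post, chain and board.
; Overlap begin sets each instance's color parameter to white or near-white, and overlap end restores hardcoded brown and gray base colors.
; The overlap events apply no filter on the overlapping actor.
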(event OnComponentBeginOverlap(highlightBox)
  (params (OtherActor :type Actor%20Object%20Reference) (OtherComp :type Primitive%20Component%20Object%20Reference) (OtherBodyIndex :type Integer) (bFromSweep :type Boolean) (SweepResult :type Hit%20Result%20Structure%20%28by%20ref%29))
  ;[1 1 1] set to highlight color
  (Utilities|FlowControl|Sequence
    (:then_0
      (Rendering|Material|SetVectorParameterValue (Variables|Default|GetDynamicPost) "post" "(R=0.989000,G=0.989000,B=0.989000,A=1.000000)" :!class /Script/Engine.MaterialInstanceDynamic))
    (:then_1
      (Rendering|Material|SetVectorParameterValue (Variables|Default|GetDynamicChain) "chain" "(R=1.000000,G=1.000000,B=1.000000,A=1.000000)" :!class /Script/Engine.MaterialInstanceDynamic))
    (:then_2
      (Rendering|Material|SetVectorParameterValue (Variables|Default|GetDynamicBoard) "board" "(R=1.000000,G=1.000000,B=1.000000,A=1.000000)" :!class /Script/Engine.MaterialInstanceDynamic))))

(event OnComponentEndOverlap(highlightBox)
  (params (OtherActor :type Actor%20Object%20Reference) (OtherComp :type Primitive%20Component%20Object%20Reference) (OtherBodyIndex :type Integer))
  ;[1 1 1] set back to proper color
  (Utilities|FlowControl|Sequence
    (:then_0
      (Rendering|Material|SetVectorParameterValue (Variables|Default|GetDynamicPost) "post" "(R=0.084000,G=0.036960,B=0.016800,A=1.000000)" :!class /Script/Engine.MaterialInstanceDynamic))
    (:then_1
      (Rendering|Material|SetVectorParameterValue (Variables|Default|GetDynamicChain) "chain" "(R=0.173000,G=0.173000,B=0.173000,A=1.000000)" :!class /Script/Engine.MaterialInstanceDynamic))
    (:then_2
      (Rendering|Material|SetVectorParameterValue (Variables|Default|GetDynamicBoard) "board" "(R=0.179000,G=0.096700,B=0.057000,A=1.000000)" :!class /Script/Engine.MaterialInstanceDynamic))))

(fn ConstructionScript
  (bind _openingsign (Variables|Default|GetopeningSign))
  (Utilities|FlowControl|Sequence
    (:then_0
      (bind _returnvalue (Rendering|Material|CreateDynamicMaterialInstance _openingsign 0 0 :!class /Script/Engine.PrimitiveComponent))
      (Variables|Default|SetDynamicPost _returnvalue))
    (:then_1
      (bind _returnvalue_2 (Rendering|Material|CreateDynamicMaterialInstance _openingsign 1 0 :!class /Script/Engine.PrimitiveComponent))
      (Variables|Default|SetDynamicChain _returnvalue_2))
    (:then_2
      (bind _returnvalue_3 (Rendering|Material|CreateDynamicMaterialInstance _openingsign 2 0 :!class /Script/Engine.PrimitiveComponent))
      (Variables|Default|SetDynamicBoard _returnvalue_3))))