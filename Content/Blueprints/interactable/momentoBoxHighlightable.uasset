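; Interactable memento box that highlights when something overlaps its HighlightBox trigger.
; The construction script creates dynamic material instances for the main wood, detail wood and hinge slots of the MomentoBox mesh.
; Begin overlap sets their wood and gold color parameters to near white, and end overlap restores hard-coded original colors, with no filter on the overlapping actor.
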(event OnComponentBeginOverlap(highlightBox)
  (params (OtherActor :type Actor%20Object%20Reference) (OtherComp :type Primitive%20Component%20Object%20Reference) (OtherBodyIndex :type Integer) (bFromSweep :type Boolean) (SweepResult :type Hit%20Result%20Structure%20%28by%20ref%29))
  ;[1 1 1] set to highlight color
  (Utilities|FlowControl|Sequence
    (:then_0
      (Rendering|Material|SetVectorParameterValue (Variables|Default|GetDynamicBoxMain) "wood" "(R=0.989000,G=0.989000,B=0.989000,A=1.000000)" :!class /Script/Engine.MaterialInstanceDynamic))
    (:then_1
      (Rendering|Material|SetVectorParameterValue (Variables|Default|GetDynamicBoxDetail) "wood" "(R=1.000000,G=1.000000,B=1.000000,A=1.000000)" :!class /Script/Engine.MaterialInstanceDynamic))
    (:then_2
      (Rendering|Material|SetVectorParameterValue (Variables|Default|GetDynamicBoxHinge) "gold" "(R=1.000000,G=1.000000,B=1.000000,A=1.000000)" :!class /Script/Engine.MaterialInstanceDynamic))))

(event OnComponentEndOverlap(highlightBox)
  (params (OtherActor :type Actor%20Object%20Reference) (OtherComp :type Primitive%20Component%20Object%20Reference) (OtherBodyIndex :type Integer))
  ;[1 1 1] set back to proper color
  (Utilities|FlowControl|Sequence
    (:then_0
      (Rendering|Material|SetVectorParameterValue (Variables|Default|GetDynamicBoxMain) "wood" "(R=0.208000,G=0.081000,B=0.059900,A=1.000000)" :!class /Script/Engine.MaterialInstanceDynamic))
    (:then_1
      (Rendering|Material|SetVectorParameterValue (Variables|Default|GetDynamicBoxDetail) "wood" "(R=0.124000,G=0.049900,B=0.037000,A=1.000000)" :!class /Script/Engine.MaterialInstanceDynamic))
    (:then_2
      (Rendering|Material|SetVectorParameterValue (Variables|Default|GetDynamicBoxHinge) "gold" "(R=0.402000,G=0.339000,B=0.130000,A=1.000000)" :!class /Script/Engine.MaterialInstanceDynamic))))

(fn ConstructionScript
  (bind _momentobox (Variables|Default|GetmomentoBox))
  (Utilities|FlowControl|Sequence
    (:then_0
      (bind _returnvalue (Rendering|Material|CreateDynamicMaterialInstance _momentobox 0 0 :!class /Script/Engine.PrimitiveComponent))
      (Variables|Default|SetDynamicBoxMain _returnvalue))
    (:then_1
      (bind _returnvalue_2 (Rendering|Material|CreateDynamicMaterialInstance _momentobox 1 0 :!class /Script/Engine.PrimitiveComponent))
      (Variables|Default|SetDynamicBoxDetail _returnvalue_2))
    (:then_2
      (bind _returnvalue_3 (Rendering|Material|CreateDynamicMaterialInstance _momentobox 2 0 :!class /Script/Engine.PrimitiveComponent))
      (Variables|Default|SetDynamicBoxHinge _returnvalue_3))))