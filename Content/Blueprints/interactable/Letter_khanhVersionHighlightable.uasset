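; Interactable letter Blueprint that highlights when something overlaps its highlight box.
; The construction script creates a dynamic material instance on the EndLetter component and stores it as DynamicLetter.
; Overlap begin sets the "letter" vector parameter to near-white, and overlap end restores its dark teal color.
; Tick watches the Checked flag, destroying the highlight box and restoring the normal color once it is true.
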(event OnComponentBeginOverlap(highlightBox)
  (params (OtherActor :type Actor%20Object%20Reference) (OtherComp :type Primitive%20Component%20Object%20Reference) (OtherBodyIndex :type Integer) (bFromSweep :type Boolean) (SweepResult :type Hit%20Result%20Structure%20%28by%20ref%29))
  ;[1 1 1] set to highlight color
  (Rendering|Material|SetVectorParameterValue (Variables|Default|GetDynamicLetter) "letter" "(R=0.989000,G=0.989000,B=0.989000,A=1.000000)" :!class /Script/Engine.MaterialInstanceDynamic))

(event OnComponentEndOverlap(highlightBox)
  (params (OtherActor :type Actor%20Object%20Reference) (OtherComp :type Primitive%20Component%20Object%20Reference) (OtherBodyIndex :type Integer))
  ;[1 1 1] set back to proper color
  (Rendering|Material|SetVectorParameterValue (Variables|Default|GetDynamicLetter) "letter" "(R=0.109804,G=0.294118,B=0.294118,A=1.000000)" :!class /Script/Engine.MaterialInstanceDynamic))

(event EventTick
  (params (DeltaSeconds :type Float%20%28single-precision%29))
  (if (Variables|Default|Getchecked)
    (Components|DestroyComponent (Variables|Default|GethighlightBox))
    ;[1 1 1] set back to proper color
    (Rendering|Material|SetVectorParameterValue (Variables|Default|GetDynamicLetter) "letter" "(R=0.109804,G=0.294118,B=0.294118,A=1.000000)" :!class /Script/Engine.MaterialInstanceDynamic)))

(fn ConstructionScript
  (bind _returnvalue (Rendering|Material|CreateDynamicMaterialInstance (Variables|Default|GetendLetter) 0 0 :!class /Script/Engine.PrimitiveComponent))
  (Variables|Default|SetDynamicLetter _returnvalue))