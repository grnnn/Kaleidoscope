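; Interactable ending letter that highlights when something overlaps its HighlightBox.
; The construction script creates dynamic material instances for the EndLetter's base and text material slots.
; Overlap begin sets a white base and highlighted letter texture, and overlap end restores the normal color and texture.
; Tick watches a Check flag and, while it is true, calls DestroyComponent and applies the same restore.
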(event OnComponentBeginOverlap(HighlightBox)
  (params (OtherActor :type Actor%20Object%20Reference) (OtherComp :type Primitive%20Component%20Object%20Reference) (OtherBodyIndex :type Integer) (bFromSweep :type Boolean) (SweepResult :type Hit%20Result%20Structure%20%28by%20ref%29))
  ;[1 1 1] set highlight color
  (Utilities|FlowControl|Sequence
    (:then_0
      (Rendering|Material|SetVectorParameterValue (Variables|Default|GetDynamicBase) "base" "(R=1.000000,G=1.000000,B=1.000000,A=1.000000)" :!class /Script/Engine.MaterialInstanceDynamic))
    (:then_1
      (Rendering|Material|SetTextureParameterValue (Variables|Default|GetDynamicText) "letter" "/Game/Model/avatarHouse/endLetterHighlight.endLetterHighlight"))))

(event OnComponentEndOverlap(HighlightBox)
  (params (OtherActor :type Actor%20Object%20Reference) (OtherComp :type Primitive%20Component%20Object%20Reference) (OtherBodyIndex :type Integer))
  ;[1 1 1] set back to proper color
  (Utilities|FlowControl|Sequence
    (:then_0
      (Rendering|Material|SetVectorParameterValue (Variables|Default|GetDynamicBase) "base" "(R=0.839216,G=0.831373,B=0.725490,A=0.000000)" :!class /Script/Engine.MaterialInstanceDynamic))
    (:then_1
      (Rendering|Material|SetTextureParameterValue (Variables|Default|GetDynamicText) "letter" "/Game/Model/avatarHouse/endLetter2.endLetter2"))))

(event EventTick
  (params (DeltaSeconds :type Float%20%28single-precision%29))
  (if (Variables|Default|Getcheck)
    (Components|DestroyComponent)
    ;[1 1 1] set back to proper color
    (Utilities|FlowControl|Sequence
      (:then_0
        (Rendering|Material|SetVectorParameterValue (Variables|Default|GetDynamicBase) "base" "(R=0.839216,G=0.831373,B=0.725490,A=0.000000)" :!class /Script/Engine.MaterialInstanceDynamic))
      (:then_1
        (Rendering|Material|SetTextureParameterValue (Variables|Default|GetDynamicText) "letter" "/Game/Model/avatarHouse/endLetter2.endLetter2")))))

(fn ConstructionScript
  (bind _endletter (Variables|Default|GetendLetter))
  (Utilities|FlowControl|Sequence
    (:then_0
      (bind _returnvalue (Rendering|Material|CreateDynamicMaterialInstance _endletter 0 0 :!class /Script/Engine.PrimitiveComponent))
      (Variables|Default|SetDynamicBase _returnvalue))
    (:then_1
      (bind _returnvalue_2 (Rendering|Material|CreateDynamicMaterialInstance _endletter 1 0 :!class /Script/Engine.PrimitiveComponent))
      (Variables|Default|SetDynamicText _returnvalue_2))))