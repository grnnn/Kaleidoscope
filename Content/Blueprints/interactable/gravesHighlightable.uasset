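; Interactable pair of graves, Aldo's and Luna's, that highlights while something overlaps its HighlightBox.
; The construction script creates dynamic material instances for the base and text slots of each grave mesh.
; Begin overlap turns both bases white and swaps in highlight name textures, and end overlap restores the dark gray and normal textures.
; Overlaps are not filtered by actor, and both graves always change together.
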(event OnComponentBeginOverlap(HighlightBox)
  (params (OtherActor :type Actor%20Object%20Reference) (OtherComp :type Primitive%20Component%20Object%20Reference) (OtherBodyIndex :type Integer) (bFromSweep :type Boolean) (SweepResult :type Hit%20Result%20Structure%20%28by%20ref%29))
  ;[1 1 1] set highlight color
  (Utilities|FlowControl|Sequence
    (:then_0
      (Rendering|Material|SetVectorParameterValue (Variables|Default|GetDynamicBaseA) "base" "(R=1.000000,G=1.000000,B=1.000000,A=1.000000)" :!class /Script/Engine.MaterialInstanceDynamic))
    (:then_1
      (Rendering|Material|SetTextureParameterValue (Variables|Default|GetDynamicTextA) "aldo" "/Game/Model/graveyard/AldoGraveHighlight.AldoGraveHighlight"))
    (:then_2
      (Rendering|Material|SetTextureParameterValue (Variables|Default|GetDynamicTextL) "luna" "/Game/Model/graveyard/LunaGraveHighlight.LunaGraveHighlight"))))

(event OnComponentEndOverlap(HighlightBox)
  (params (OtherActor :type Actor%20Object%20Reference) (OtherComp :type Primitive%20Component%20Object%20Reference) (OtherBodyIndex :type Integer))
  ;[1 1 1] set back to proper color
  (Utilities|FlowControl|Sequence
    (:then_0
      (Rendering|Material|SetVectorParameterValue (Variables|Default|GetDynamicBaseA) "base" "(R=0.231000,G=0.231000,B=0.231000,A=1.000000)" :!class /Script/Engine.MaterialInstanceDynamic))
    (:then_1
      (Rendering|Material|SetTextureParameterValue (Variables|Default|GetDynamicTextA) "aldo" "/Game/Model/graveyard/AldoGrave.AldoGrave"))
    (:then_2
      (Rendering|Material|SetTextureParameterValue (Variables|Default|GetDynamicTextL) "luna" "/Game/Model/graveyard/LunaGrave.LunaGrave"))))

(fn ConstructionScript
  (bind _lunagrave (Variables|Default|GetlunaGrave))
  (bind _aldograve (Variables|Default|GetaldoGrave))
  (Utilities|FlowControl|Sequence
    (:then_0
      (bind _returnvalue (Rendering|Material|CreateDynamicMaterialInstance _aldograve 0 0 :!class /Script/Engine.PrimitiveComponent))
      (Variables|Default|SetDynamicBaseA _returnvalue))
    (:then_1
      (bind _returnvalue_2 (Rendering|Material|CreateDynamicMaterialInstance _aldograve 1 0 :!class /Script/Engine.PrimitiveComponent))
      (Variables|Default|SetDynamicTextA _returnvalue_2))
    (:then_2
      (bind _returnvalue_3 (Rendering|Material|CreateDynamicMaterialInstance _lunagrave 0 0 :!class /Script/Engine.PrimitiveComponent))
      (Variables|Default|SetDynamicBaseL _returnvalue_3))
    (:then_3
      (bind _returnvalue_4 (Rendering|Material|CreateDynamicMaterialInstance _lunagrave 1 0 :!class /Script/Engine.PrimitiveComponent))
      (Variables|Default|SetDynamicTextL _returnvalue_4))))