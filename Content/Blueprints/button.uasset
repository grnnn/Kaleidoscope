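; Button actor that acts as an overlap trigger, signaling when something enters or leaves it.
; Begin and end overlap set the Intrigger flag, then share one branch that calls the Buttontrue or Buttonfalse event dispatcher.
; Both paths toggle the TextRender1 label's visibility, and the overlapping actor is not filtered.
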(event EventActorBeginOverlap
  (params (OtherActor :type Actor%20Object%20Reference))
  (Variables|Default|Setintrigger true)
  (if (Variables|Default|Getintrigger)
    (Rendering|ToggleVisibility (Variables|Default|GetTextRender1) false)
    (Default|CallButtontrue)
    (else
      (Rendering|ToggleVisibility (Variables|Default|GetTextRender1) false)
      (Default|CallButtonfalse))))

(event EventActorEndOverlap
  (params (OtherActor :type Actor%20Object%20Reference))
  (Variables|Default|Setintrigger false)
  (if (Variables|Default|Getintrigger)
    (Rendering|ToggleVisibility (Variables|Default|GetTextRender1) false)
    (Default|CallButtontrue)
    (else
      (Rendering|ToggleVisibility (Variables|Default|GetTextRender1) false)
      (Default|CallButtonfalse))))

(fn ConstructionScript)