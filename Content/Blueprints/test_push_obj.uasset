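; Test actor for a physics object that the player can push with the F key.
; Entering Box1 with a "player"-tagged actor enables input, highlights StaticMesh1 through custom depth and prints a prompt; leaving reverses the input and highlight.
; Pressing F while inside applies one large force along the controller's yaw-only forward direction.
; The nodes that would enable physics simulation are unconnected, so the graph never turns it on.
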(event OnComponentBeginOverlap(Box1)
  (params (OtherActor :type Actor%20Object%20Reference) (OtherComp :type Primitive%20Component%20Object%20Reference) (OtherBodyIndex :type Integer) (bFromSweep :type Boolean) (SweepResult :type Hit%20Result%20Structure%20%28by%20ref%29))
  ;[1 1 1] Active/Deactive highlight and input  when player get near the object
  (if (Actor|ActorHasTag OtherActor "player")
    (Variables|Default|SetisTrigger true)
    (Rendering|SetRenderCustomDepth (Variables|Default|GetStaticMesh1) true)
    (Input|EnableInput (Game|GetPlayerController 0))
    (Development|PrintString "Press F to push" true true "(R=1.000000,G=0.036913,B=0.000000,A=1.000000)")))

(event OnComponentEndOverlap(Box1)
  (params (OtherActor :type Actor%20Object%20Reference) (OtherComp :type Primitive%20Component%20Object%20Reference) (OtherBodyIndex :type Integer))
  ;[1 1 1] Active/Deactive highlight and input  when player get near the object
  (if (Actor|ActorHasTag OtherActor "player")
    (Variables|Default|SetisTrigger false)
    (Rendering|SetRenderCustomDepth (Variables|Default|GetStaticMesh1) false)
    (Input|DisableInput (Game|GetPlayerController 0))))

(event EventTick
  (params (DeltaSeconds :type Float%20%28single-precision%29))
  ;[1 1 1] trash - will delete
)

(event EventBeginPlay
  ;[1 1 1] trash - will delete
)

(event Input|KeyboardEvents|F
  (:Pressed
    ;[1 1 1] Apply force to the object in the direction player facing (forward direction)
    (if (Variables|Default|GetisTrigger)
      (Physics|AddForce (Variables|Default|GetStaticMesh1) (* (Math|Vector|GetForwardVector (Class|KismetMathLibrary|MakeRot 0.0 (.Yaw (Class|KismetMathLibrary|BreakRot (Pawn|GetControlRotation (Game|GetPlayerController 0) :!class /Script/Engine.Controller))) 0.0)) 1e+08) "None"))))

(fn ConstructionScript)