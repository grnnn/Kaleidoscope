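; CameraTurn2 is a special camera actor that turns to follow the player once triggered.
; An overlap on Box1 sets an active flag, which nothing in the graph clears.
; While active, Tick sets Camera1's world rotation to the look-at yaw toward player character 0, holding pitch and roll at zero.
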(event OnComponentBeginOverlap(Box1)
  (params (OtherActor :type Actor%20Object%20Reference) (OtherComp :type Primitive%20Component%20Object%20Reference) (OtherBodyIndex :type Integer) (bFromSweep :type Boolean) (SweepResult :type Hit%20Result%20Structure%20%28by%20ref%29))
  (Variables|Default|SetisActive true))

(event EventTick
  (params (DeltaSeconds :type Float%20%28single-precision%29))
  (bind _camera1 (Variables|Default|GetCamera1))
  (if (Variables|Default|GetisActive)
    (Transformation|SetWorldRotation _camera1 (Class|KismetMathLibrary|MakeRot 0.0 (.Yaw (Class|KismetMathLibrary|BreakRot (Math|Rotator|FindLookatRotation (Transformation|GetWorldLocation _camera1) (Transformation|GetActorLocation (Game|GetPlayerCharacter 0))))) 0.0) false)))

(fn ConstructionScript)