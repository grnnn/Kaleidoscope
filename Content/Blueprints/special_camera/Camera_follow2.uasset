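; Special follow camera that mirrors the main character's view.
; Every Tick it casts player 0's character to MyCharacter and copies the world transform of that character's FollowCamera onto itself, without sweep or smoothing.
; An unconnected transform that would offset the location along world X and Z is left unused.
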(event EventTick
  (params (DeltaSeconds :type Float%20%28single-precision%29))
  ;[1 1 1] Make this camera to follow the main character
  (bind _asmy_character (Utilities|Casting|CastToMyCharacter (Game|GetPlayerCharacter 0)))
  (Transformation|SetWorldTransform (Transformation|GetWorldTransform (Variables|/Script/Kaleidoscope.KaleidoscopeCharacter|GetFollowCamera _asmy_character)) false))

(fn ConstructionScript)