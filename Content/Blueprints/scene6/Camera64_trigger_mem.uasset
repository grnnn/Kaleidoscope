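; Scene 6 camera trigger that glides Camera1 by fixed location and rotation steps while MemTriggered is set and MemDone is not.
; BeginPlay derives each step as a thousandth of the offset to TargetLoc and TargetRot, with the Z component negated.
; Tick adds the steps every frame, so speed depends on frame rate.
; Nothing here sets either flag or stops at the target.
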(event EventBeginPlay
  (bind _target_rot (Variables|Default|Gettarget_rot))
  (bind _camera1 (Variables|Default|GetCamera1))
  (bind _target_loc (Variables|Default|Gettarget_loc))
  (bind _returnvalue (Transformation|GetWorldRotation _camera1))
  (bind (_pitch _yaw _roll) (Class|KismetMathLibrary|BreakRot _target_rot))
  (bind _returnvalue_2 (Transformation|GetWorldLocation _camera1))
  (bind (_pitch_2 _yaw_2 _roll_2) (Class|KismetMathLibrary|BreakRot _returnvalue))
  (bind _returnvalue_3 (- _target_loc _returnvalue_2))
  (bind (_x _y _z) (Math|Vector|BreakVector _returnvalue_3))
  (Variables|Default|Setdelta_loc (Math|Vector|MakeVector (/ _x 1e+03) (/ _y 1e+03) (/ (* _z -1.0) 1e+03)))
  (Variables|Default|Setdelta_rot (Class|KismetMathLibrary|MakeRot (/ (- _pitch _pitch_2) 1e+03) (/ (- _yaw _yaw_2) 1e+03) (/ (- _roll _roll_2) 1e+03))))

(event EventTick
  (params (DeltaSeconds :type Float%20%28single-precision%29))
  (bind _camera1 (Variables|Default|GetCamera1))
  (bind _delta_rot (Variables|Default|Getdelta_rot))
  (bind _returnvalue (Transformation|GetWorldRotation _camera1))
  (bind (_pitch _yaw _roll) (Class|KismetMathLibrary|BreakRot _delta_rot))
  (bind (_pitch_2 _yaw_2 _roll_2) (Class|KismetMathLibrary|BreakRot _returnvalue))
  (if (not (Variables|Default|Getmem_done))
    (if (Variables|Default|Getmem_triggered)
      (Transformation|SetWorldLocationAndRotation _camera1 (+ (Transformation|GetWorldLocation _camera1) (Variables|Default|Getdelta_loc)) (Class|KismetMathLibrary|MakeRot (+ _pitch_2 _pitch) (+ _yaw_2 _yaw) (+ _roll_2 _roll)) false))))

(fn ConstructionScript)