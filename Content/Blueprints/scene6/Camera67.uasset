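; Camera67 is a scene 6 Blueprint that turns its Camera1 component to face the player character.
; While Triggered is true, each Tick computes a look-at rotation from Camera1 to the player and applies only its yaw, holding pitch and roll at zero.
; Nothing in this file sets Triggered, and a yaw offset calculation is left unused.
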(event EventTick
  (params (DeltaSeconds :type Float%20%28single-precision%29))
  (bind _camera1 (Variables|Default|GetCamera1))
  (if (Variables|Default|Gettriggered)
    (Transformation|SetWorldRotation _camera1 (Class|KismetMathLibrary|MakeRot 0.0 (.Yaw (Class|KismetMathLibrary|BreakRot (Math|Rotator|FindLookatRotation (Transformation|GetWorldLocation _camera1) (Transformation|GetActorLocation (Game|GetPlayerCharacter 0))))) 0.0) false)))

(fn ConstructionScript)