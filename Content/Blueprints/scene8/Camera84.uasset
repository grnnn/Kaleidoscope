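; Scene 8 camera Blueprint that glides Camera1 toward a target location once a "Mem" trigger flag is set.
; BeginPlay divides the offset to TargetLoc by Delta to get a fixed step.
; Tick adds that step, unscaled by frame time, while MemDone is false and the camera's X and Z are both below the target's.
; Neither flag is set here, and an unconnected comparison remains unused.
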(event EventBeginPlay
  (bind _camera1 (Variables|Default|GetCamera1))
  (bind _target_loc (Variables|Default|Gettarget_loc))
  (bind _delta (Variables|Default|Getdelta))
  (bind _returnvalue (Transformation|GetWorldLocation _camera1))
  (bind _returnvalue_2 (- _target_loc _returnvalue))
  (bind (_x _y _z) (Math|Vector|BreakVector _returnvalue_2))
  (Variables|Default|Setdelta_loc (Math|Vector|MakeVector (/ _x _delta) (/ _y _delta) (/ (* _z 1.0) _delta))))

(event EventTick
  (params (DeltaSeconds :type Float%20%28single-precision%29))
  (bind _camera1 (Variables|Default|GetCamera1))
  (bind _target_loc (Variables|Default|Gettarget_loc))
  (bind (_x _y _z) (Math|Vector|BreakVector _target_loc))
  (bind _returnvalue (Transformation|GetWorldLocation _camera1))
  (bind (_x_2 _y_2 _z_2) (Math|Vector|BreakVector _returnvalue))
  (if (not (Variables|Default|Getmem_done))
    (if (Variables|Default|Getmem_triggered)
      (if (and (< _z_2 _z) (< _x_2 _x))
        (Transformation|SetWorldLocation _camera1 (+ _returnvalue (Variables|Default|Getdelta_loc)) false)))))

(fn ConstructionScript)