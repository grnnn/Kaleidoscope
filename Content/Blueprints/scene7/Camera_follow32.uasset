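; Camera actor for scene7 that follows the player's main character.
; On BeginPlay it casts player character 0 to MyCharacter and attaches to that character's SpringArm1 with SnapToTarget, so the spring arm drives the follow motion.
; There is no per-frame logic; the leftover transform nodes are unused and never run.
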(event EventBeginPlay
  ;[1 1 1] Make this camera to follow the main character
  (bind _asmy_character (Utilities|Casting|CastToMyCharacter (Game|GetPlayerCharacter 0)))
  (Class|SceneComponent|Attachto (Variables|/Game/Blueprints/MyCharacter.MyCharacter_C|GetSpringArm1 _asmy_character) "None" "SnapToTarget" true))

(fn ConstructionScript)