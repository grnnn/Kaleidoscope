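; Scripted camera Blueprint for scene7 that zooms Camera1 to a target point, then raises it vertically.
; BeginPlay precomputes fixed per-tick steps from the start location, TargetZoom, TargetUP and DeltaDetermineZoom.
; While MemTriggered is set, Tick moves the camera until its X or Y reaches TargetZoom, then lifts it to a hard-coded height.
; Movement ignores delta time, so its speed depends on frame rate.
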(event EventTick
  (params (DeltaSeconds :type Float%20%28single-precision%29))
  (bind _camera1 (Variables|Default|GetCamera1))
  (bind _targetzoom (Variables|Default|GettargetZoom))
  (bind _camera1_2 (Variables|Default|GetCamera1))
  (bind (_x _y) (Math|Vector|BreakVector _targetzoom))
  (bind _returnvalue (Transformation|GetWorldLocation _camera1_2))
  (bind _returnvalue_2 (Transformation|GetWorldLocation _camera1))
  (bind (_x_2 _y_2 _z) (Math|Vector|BreakVector _returnvalue_2))
  (if (Variables|Default|Getmem_triggered)
    (if (and (< _x_2 _x) (< _y_2 _y))
      (Transformation|SetWorldLocation _camera1_2 (+ _returnvalue (Variables|Default|Getdelta_zoom)) false)
      (elif (< _z 3.8e+02)
        (Transformation|SetWorldLocation _camera1_2 (+ _returnvalue (Variables|Default|Getdelta_up)) false)))))

(event EventBeginPlay
  (bind _targetzoom (Variables|Default|GettargetZoom))
  (bind _camera1 (Variables|Default|GetCamera1))
  (bind _delta_determine_zoom (Variables|Default|Getdelta_determine_zoom))
  (bind _returnvalue (Transformation|GetWorldLocation _camera1))
  (bind (_x _y _z) (Math|Vector|BreakVector _targetzoom))
  (bind (_x_2 _y_2 _z_2) (Math|Vector|BreakVector _returnvalue))
  (Variables|Default|Setdelta_zoom (Math|Vector|MakeVector (/ (- _x _x_2) _delta_determine_zoom) (/ (- _y _y_2) _delta_determine_zoom) (/ (- _z _z_2) _delta_determine_zoom)))
  (Variables|Default|Setdelta_up (Math|Vector|MakeVector 0.0 0.0 (/ (- (.Z (Math|Vector|BreakVector (Variables|Default|GettargetUP))) (.Z (Math|Vector|BreakVector (Variables|Default|GettargetZoom)))) _delta_determine_zoom))))

(fn ConstructionScript)