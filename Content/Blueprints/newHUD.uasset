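; HUD Blueprint with two timed text slots, though its DrawHUD event is empty, so this graph draws nothing.
; ShowText and ShowText2 each store a string and screen position, then clear the string after the given delay.
; Disconnected leftover logic holds a hardcoded letter from Mom to Alina, drawn line by line, plus an F-key check on its Text1On flag.
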(event EventDrawHUD
  (params (SizeX :type Integer) (SizeY :type Integer)))

(event EventShowText2
  (params (Text2 :type String) (TextX2 :type Float%20%28single-precision%29) (TextY2 :type Float%20%28single-precision%29) (Duration2 :type Float%20%28single-precision%29))
  (Variables|Default|SetText2 Text2)
  (Variables|Default|SetTextX2 TextX2)
  (Variables|Default|SetTextY2 TextY2)
  (Utilities|FlowControl|Delay 0 Duration2)
  (Variables|Default|SetText2 ""))

(event EventShowText
  (params (Text :type String) (TextX :type Float%20%28single-precision%29) (TextY :type Float%20%28single-precision%29) (Duration :type Float%20%28single-precision%29) (Text2 :type String) (Duration2 :type Float%20%28single-precision%29))
  (Variables|Default|SetText Text)
  (Variables|Default|SetTextX TextX)
  (Variables|Default|SetTextY TextY)
  (Utilities|FlowControl|Delay 0 Duration2)
  (Variables|Default|SetText "  "))

(fn ConstructionScript)