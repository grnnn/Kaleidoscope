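; Test Blueprint for a physics object that the player picks up by holding F.
; Overlapping Box1 with a "player"-tagged actor enables input, outlines the mesh through custom depth and prints a prompt.
; Pressing F stops physics, attaches the root to the character mesh socket "newq", ignores Pawn collision and raises the mesh.
; Releasing F restores physics and Pawn blocking, with no explicit detach.
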(event OnComponentBeginOverlap(Box1)
  (params (OtherActor :type Actor%20Object%20Reference) (OtherComp :type Primitive%20Component%20Object%20Reference) (OtherBodyIndex :type Integer) (bFromSweep :type Boolean) (SweepResult :type Hit%20Result%20Structure%20%28by%20ref%29))
  ;[1 1 1] Active/Deactive highlight and input  when player get near the object
  (if (Actor|ActorHasTag OtherActor "player")
    (Variables|Default|SetisTrigger true)
    (Rendering|SetRenderCustomDepth (Variables|Default|GetStaticMesh1) true)
    (Input|EnableInput (Game|GetPlayerController 0))
    (Development|PrintString "Press F to pickup" true true "(R=1.000000,G=0.036913,B=0.000000,A=1.000000)")))

(event OnComponentEndOverlap(Box1)
  (params (OtherActor :type Actor%20Object%20Reference) (OtherComp :type Primitive%20Component%20Object%20Reference) (OtherBodyIndex :type Integer))
  ;[1 1 1] Active/Deactive highlight and input  when player get near the object
  (if (Actor|ActorHasTag OtherActor "player")
    (Variables|Default|SetisTrigger false)
    (Rendering|SetRenderCustomDepth (Variables|Default|GetStaticMesh1) false)
    (Input|DisableInput (Game|GetPlayerController 0))))

(event EventTick
  (params (DeltaSeconds :type Float%20%28single-precision%29))
  ;[1 1 1] trash - will delete
)

(event EventBeginPlay
  ;[1 1 1] trash - will delete
)

(event Input|KeyboardEvents|F
  (bind _staticmesh1 (Variables|Default|GetStaticMesh1))
  (bind _staticmesh1_2 (Variables|Default|GetStaticMesh1))
  (bind _returnvalue (Transformation|GetWorldLocation _staticmesh1))
  (bind (_x _y _z) (Math|Vector|BreakVector _returnvalue))
  ;[1 1 1] Pick up object
  (:Pressed
    (if (Variables|Default|GetisTrigger)
      (Physics|SetSimulatePhysics _staticmesh1_2 false)
      (Class|Actor|AttachRootComponentto (Variables|/Script/Engine.Character|GetMesh (Game|GetPlayerCharacter 0)) "newq" "KeepWorldPosition" true)
      (Collision|SetCollisionResponsetoChannel _staticmesh1 "ECC_Pawn" "ECR_Ignore")
      (Transformation|SetWorldLocation _staticmesh1 (Math|Vector|MakeVector _x _y (+ _z 5e+01)) false)))
  (:Released
    (Physics|SetSimulatePhysics _staticmesh1_2 true)
    (Collision|SetCollisionResponsetoChannel (Variables|Default|GetStaticMesh1) "ECC_Pawn" "ECR_Block")))

(fn ConstructionScript)