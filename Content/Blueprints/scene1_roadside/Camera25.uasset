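; Camera25 is a scene capture camera in the roadside scene that shifts its image saturation or slowly zooms in.
; While ChangeSat is set, Tick raises film saturation toward 0.3 by rebuilding the capture's post-process settings.
; Otherwise, MemoryTriggered narrows the field of view each tick down to 50 degrees.
; The intended countdown delay before the zoom is bypassed by an always-true branch, leaving the Counter decrement unreachable.
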(event EventTick
  (params (DeltaSeconds :type Float%20%28single-precision%29))
  (bind _scenecapture2d1 (Variables|Default|GetSceneCapture2D1))
  (bind _scenecapture2d1_2 (Variables|Default|GetSceneCapture2D1))
  ;[1 1 1] Saturation Change
  (if (Variables|Default|GetChangeSat)
    (if (< (Variables|Default|GetsaturationValue) 0.3)
      (Variables|Default|SetsaturationValue (- (Variables|Default|GetsaturationValue) -0.005))
      (Variables|/Script/Engine.SceneCaptureComponent2D|SetPostProcessSettings _scenecapture2d1_2 (Utilities|Struct|MakePostProcessSettings (.bOverride_FilmWhitePoint (Utilities|Struct|BreakPostProcessSettings (Variables|/Script/Engine.SceneCaptureComponent2D|GetPostProcessSettings _scenecapture2d1_2))) true (.bOverride_FilmChannelMixerRed (Utilities|Struct|BreakPostProcessSettings (Variables|/Script/Engine.SceneCaptureComponent2D|GetPostProcessSettings _scenecapture2d1_2))) (.bOverride_FilmChannelMixerGreen (Utilities|Struct|BreakPostProcessSettings (Variables|/Script/Engine.SceneCaptureComponent2D|GetPostProcessSettings _scenecapture2d1_2))) (.bOverride_FilmChannelMixerBlue (Utilities|Struct|BreakPostProcessSettings (Variables|/Script/Engine.SceneCaptureComponent2D|GetPostProcessSettings _scenecapture2d1_2))) (.bOverride_FilmContrast (Utilities|Struct|BreakPostProcessSettings (Variables|/Script/Engine.SceneCaptureComponent2D|GetPostProcessSettings _scenecapture2d1_2))) (.bOverride_FilmDynamicRange (Utilities|Struct|BreakPostProcessSettings (Variables|/Script/Engine.SceneCaptureComponent2D|GetPostProcessSettings _scenecapture2d1_2))) (.bOverride_FilmHealAmount (Utilities|Struct|BreakPostProcessSettings (Variables|/Script/Engine.SceneCaptureComponent2D|GetPostProcessSettings _scenecapture2d1_2))) (.bOverride_FilmToeAmount (Utilities|Struct|BreakPostProcessSettings (Variables|/Script/Engine.SceneCaptureComponent2D|GetPostProcessSettings _scenecapture2d1_2))) (.bOverride_FilmShadowTint (Utilities|Struct|BreakPostProcessSettings (Variables|/Script/Engine.SceneCaptureComponent2D|GetPostProcessSettings _scenecapture2d1_2))) (.bOverride_FilmShadowTintBlend (Utilities|Struct|BreakPostProcessSettings (Variables|/Script/Engine.SceneCaptureComponent2D|GetPostProcessSettings _scenecapture2d1_2))) (.bOverride_FilmShadowTintAmount (Utilities|Struct|BreakPostProcessSettings (Variables|/Script/Engine.SceneCaptureComponent2D|GetPostProcessSettings _scenecapture2d1_2))) (.bOverride_SceneColorTint (Utilities|Struct|BreakPostProcessSettings (Variables|/Script/Engine.SceneCaptureComponent2D|GetPostProcessSettings _scenecapture2d1_2))) (.bOverride_SceneFringeIntensity (Utilities|Struct|BreakPostProcessSettings (Variables|/Script/Engine.SceneCaptureComponent2D|GetPostProcessSettings _scenecapture2d1_2))) (.bOverride_SceneFringeSaturation (Utilities|Struct|BreakPostProcessSettings (Variables|/Script/Engine.SceneCaptureComponent2D|GetPostProcessSettings _scenecapture2d1_2))) (.bOverride_AmbientCubemapTint (Utilities|Struct|BreakPostProcessSettings (Variables|/Script/Engine.SceneCaptureComponent2D|GetPostProcessSettings _scenecapture2d1_2))) (.bOverride_AmbientCubemapIntensity (Utilities|Struct|BreakPostProcessSettings (Variables|/Script/Engine.SceneCaptureComponent2D|GetPostProcessSettings _scenecapture2d1_2))) (.bOverride_BloomIntensity (Utilities|Struct|BreakPostProcessSettings (Variables|/Script/Engine.SceneCaptureComponent2D|GetPostProcessSettings _scenecapture2d1_2))) (.bOverride_BloomThreshold (Utilities|Struct|BreakPostProcessSettings (Variables|/Script/Engine.SceneCaptureComponent2D|GetPostProcessSettings _scenecapture2d1_2))) (.bOverride_Bloom1Tint (Utilities|Struct|BreakPostProcessSettings (Variables|/Script/Engine.SceneCaptureComponent2D|GetPostProcessSettings _scenecapture2d1_2))) (.bOverride_Bloom1Size (Utilities|Struct|BreakPostProcessSettings (Variables|/Script/Engine.SceneCaptureComponent2D|GetPostProcessSettings _scenecapture2d1_2))) (.bOverride_Bloom2Size (Utilities|Struct|BreakPostProcessSettings (Variables|/Script/Engine.SceneCaptureComponent2D|GetPostProcessSettings _scenecapture2d1_2))) (.bOverride_Bloom2Tint (Utilities|Struct|BreakPostProcessSettings (Variables|/Script/Engine.SceneCaptureComponent2D|GetPostProcessSettings _scenecapture2d1_2))) (.bOverride_Bloom3Tint (Utilities|Struct|BreakPostProcessSettings (Variables|/Script/Engine.SceneCaptureComponent2D|GetPostProcessSettings _scenecapture2d1_2))) (.bOverride_Bloom3Size (Utilities|Struct|BreakPostProcessSettings (Variables|/Script/Engine.SceneCaptureComponent2D|GetPostProcessSettings _scenecapture2d1_2))) (.bOverride_Bloom4Tint (Utilities|Struct|BreakPostProcessSettings (Variables|/Script/Engine.SceneCaptureComponent2D|GetPostProcessSettings _scenecapture2d1_2))) (.bOverride_Bloom4Size (Utilities|Struct|BreakPostProcessSettings (Variables|/Script/Engine.SceneCaptureComponent2D|GetPostProcessSettings _scenecapture2d1_2))) (.bOverride_Bloom5Tint (Utilities|Struct|BreakPostProcessSettings (Variables|/Script/Engine.SceneCaptureComponent2D|GetPostProcessSettings _scenecapture2d1_2))) (.bOverride_Bloom5Size (Utilities|Struct|BreakPostProcessSettings (Variables|/Script/Engine.SceneCaptureComponent2D|GetPostProcessSettings _scenecapture2d1_2))) (.bOverride_BloomDirtMaskIntensity (Utilities|Struct|BreakPostProcessSettings (Variables|/Script/Engine.SceneCaptureComponent2D|GetPostProcessSettings _scenecapture2d1_2))) (.bOverride_BloomDirtMaskTint (Utilities|Struct|BreakPostProcessSettings (Variables|/Script/Engine.SceneCaptureComponent2D|GetPostProcessSettings _scenecapture2d1_2))) (.bOverride_BloomDirtMask (Utilities|Struct|BreakPostProcessSettings (Variables|/Script/Engine.SceneCaptureComponent2D|GetPostProcessSettings _scenecapture2d1_2))) (.bOverride_AutoExposureLowPercent (Utilities|Struct|BreakPostProcessSettings (Variables|/Script/Engine.SceneCaptureComponent2D|GetPostProcessSettings _scenecapture2d1_2))) (.bOverride_AutoExposureHighPercent (Utilities|Struct|BreakPostProcessSettings (Variables|/Script/Engine.SceneCaptureComponent2D|GetPostProcessSettings _scenecapture2d1_2))) (.bOverride_AutoExposureMinBrightness (Utilities|Struct|BreakPostProcessSettings (Variables|/Script/Engine.SceneCaptureComponent2D|GetPostProcessSettings _scenecapture2d1_2))) (.bOverride_AutoExposureMaxBrightness (Utilities|Struct|BreakPostProcessSettings (Variables|/Script/Engine.SceneCaptureComponent2D|GetPostProcessSettings _scenecapture2d1_2))) (.bOverride_AutoExposureSpeedUp (Utilities|Struct|BreakPostProcessSettings (Variables|/Script/Engine.SceneCaptureComponent2D|GetPostProcessSettings _scenecapture2d1_2))) (.bOverride_AutoExposureSpeedDown (Utilities|Struct|BreakPostProcessSettings (Variables|/Script/Engine.SceneCaptureComponent2D|GetPostProcessSettings _scenecapture2d1_2))) (.bOverride_AutoExposureBias (Utilities|Struct|BreakPostProcessSettings (Variables|/Script/Engine.SceneCaptureComponent2D|GetPostProcessSettings _scenecapture2d1_2))) (.bOverride_HistogramLogMin (Utilities|Struct|BreakPostProcessSettings (Variables|/Script/Engine.SceneCaptureComponent2D|GetPostProcessSettings _scenecapture2d1_2))) (.bOverride_HistogramLogMax (Utilities|Struct|BreakPostProcessSettings (Variables|/Script/Engine.SceneCaptureComponent2D|GetPostProcessSettings _scenecapture2d1_2))) (.bOverride_LensFlareIntensity (Utilities|Struct|BreakPostProcessSettings (Variables|/Script/Engine.SceneCaptureComponent2D|GetPostProcessSettings _scenecapture2d1_2))) (.bOverride_LensFlareTint (Utilities|Struct|BreakPostProcessSettings (Variables|/Script/Engine.SceneCaptureComponent2D|GetPostProcessSettings _scenecapture2d1_2))) (.bOverride_LensFlareTints (Utilities|Struct|BreakPostProcessSettings (Variables|/Script/Engine.SceneCaptureComponent2D|GetPostProcessSettings _scenecapture2d1_2))) (.bOverride_LensFlareBokehSize (Utilities|Struct|BreakPostProcessSettings (Variables|/Script/Engine.SceneCaptureComponent2D|GetPostProcessSettings _scenecapture2d1_2))) (.bOverride_LensFlareBokehShape (Utilities|Struct|BreakPostProcessSettings (Variables|/Script/Engine.SceneCaptureComponent2D|GetPostProcessSettings _scenecapture2d1_2))) (.bOverride_LensFlareThreshold (Utilities|Struct|BreakPostProcessSettings (Variables|/Script/Engine.SceneCaptureComponent2D|GetPostProcessSettings _scenecapture2d1_2))) (.bOverride_VignetteIntensity (Utilities|Struct|BreakPostProcessSettings (Variables|/Script/Engine.SceneCaptureComponent2D|GetPostProcessSettings _scenecapture2d1_2))) (.bOverride_VignetteColor (Utilities|Struct|BreakPostProcessSettings (Variables|/Script/Engine.SceneCaptureComponent2D|GetPostProcessSettings _scenecapture2d1_2))) (.bOverride_GrainIntensity (Utilities|Struct|BreakPostProcessSettings (Variables|/Script/Engine.SceneCaptureComponent2D|GetPostProcessSettings _scenecapture2d1_2))) (.bOverride_GrainJitter (Utilities|Struct|BreakPostProcessSettings (Variables|/Script/Engine.SceneCaptureComponent2D|GetPostProcessSettings _scenecapture2d1_2))) (.bOverride_AmbientOcclusionIntensity (Utilities|Struct|BreakPostProcessSettings (Variables|/Script/Engine.SceneCaptureComponent2D|GetPostProcessSettings _scenecapture2d1_2))) (.bOverride_AmbientOcclusionStaticFraction (Utilities|Struct|BreakPostProcessSettings (Variables|/Script/Engine.SceneCaptureComponent2D|GetPostProcessSettings _scenecapture2d1_2))) (.bOverride_AmbientOcclusionRadius (Utilities|Struct|BreakPostProcessSettings (Variables|/Script/Engine.SceneCaptureComponent2D|GetPostProcessSettings _scenecapture2d1_2))) (.bOverride_AmbientOcclusionFadeDistance (Utilities|Struct|BreakPostProcessSettings (Variables|/Script/Engine.SceneCaptureComponent2D|GetPostProcessSettings _scenecapture2d1_2))) (.bOverride_AmbientOcclusionFadeRadius (Utilities|Struct|BreakPostProcessSettings (Variables|/Script/Engine.SceneCaptureComponent2D|GetPostProcessSettings _scenecapture2d1_2))) (.bOverride_AmbientOcclusionDistance (Utilities|Struct|BreakPostProcessSettings (Variables|/Script/Engine.SceneCaptureComponent2D|GetPostProcessSettings _scenecapture2d1_2))) (.bOverride_AmbientOcclusionRadiusInWS (Utilities|Struct|BreakPostProcessSettings (Variables|/Script/Engine.SceneCaptureComponent2D|GetPostProcessSettings _scenecapture2d1_2))) (.bOverride_AmbientOcclusionPower (Utilities|Struct|BreakPostProcessSettings (Variables|/Script/Engine.SceneCaptureComponent2D|GetPostProcessSettings _scenecapture2d1_2))) (.bOverride_AmbientOcclusionBias (Utilities|Struct|BreakPostProcessSettings (Variables|/Script/Engine.SceneCaptureComponent2D|GetPostProcessSettings _scenecapture2d1_2))) (.bOverride_AmbientOcclusionQuality (Utilities|Struct|BreakPostProcessSettings (Variables|/Script/Engine.SceneCaptureComponent2D|GetPostProcessSettings _scenecapture2d1_2))) (.bOverride_AmbientOcclusionMipBlend (Utilities|Struct|BreakPostProcessSettings (Variables|/Script/Engine.SceneCaptureComponent2D|GetPostProcessSettings _scenecapture2d1_2))) (.bOverride_AmbientOcclusionMipScale (Utilities|Struct|BreakPostProcessSettings (Variables|/Script/Engine.SceneCaptureComponent2D|GetPostProcessSettings _scenecapture2d1_2))) (.bOverride_AmbientOcclusionMipThreshold (Utilities|Struct|BreakPostProcessSettings (Variables|/Script/Engine.SceneCaptureComponent2D|GetPostProcessSettings _scenecapture2d1_2))) (.bOverride_LPVIntensity (Utilities|Struct|BreakPostProcessSettings (Variables|/Script/Engine.SceneCaptureComponent2D|GetPostProcessSettings _scenecapture2d1_2))) (.bOverride_LPVWarpIntensity (Utilities|Struct|BreakPostProcessSettings (Variables|/Script/Engine.SceneCaptureComponent2D|GetPostProcessSettings _scenecapture2d1_2))) (.bOverride_LPVSize (Utilities|Struct|BreakPostProcessSettings (Variables|/Script/Engine.SceneCaptureComponent2D|GetPostProcessSettings _scenecapture2d1_2))) (.bOverride_LPVSecondaryOcclusionIntensity (Utilities|Struct|BreakPostProcessSettings (Variables|/Script/Engine.SceneCaptureComponent2D|GetPostProcessSettings _scenecapture2d1_2))) (.bOverride_LPVSecondaryBounceIntensity (Utilities|Struct|BreakPostProcessSettings (Variables|/Script/Engine.SceneCaptureComponent2D|GetPostProcessSettings _scenecapture2d1_2))) (.bOverride_LPVGeometryVolumeBias (Utilities|Struct|BreakPostProcessSettings (Variables|/Script/Engine.SceneCaptureComponent2D|GetPostProcessSettings _scenecapture2d1_2))) (.bOverride_LPVVplInjectionBias (Utilities|Struct|BreakPostProcessSettings (Variables|/Script/Engine.SceneCaptureComponent2D|GetPostProcessSettings _scenecapture2d1_2))) (.bOverride_LPVEmissiveInjectionIntensity (Utilities|Struct|BreakPostProcessSettings (Variables|/Script/Engine.SceneCaptureComponent2D|GetPostProcessSettings _scenecapture2d1_2))) (.bOverride_LPVTransmissionIntensity (Utilities|Struct|BreakPostProcessSettings (Variables|/Script/Engine.SceneCaptureComponent2D|GetPostProcessSettings _scenecapture2d1_2))) (.bOverride_IndirectLightingColor (Utilities|Struct|BreakPostProcessSettings (Variables|/Script/Engine.SceneCaptureComponent2D|GetPostProcessSettings _scenecapture2d1_2))) (.bOverride_IndirectLightingIntensity (Utilities|Struct|BreakPostProcessSettings (Variables|/Script/Engine.SceneCaptureComponent2D|GetPostProcessSettings _scenecapture2d1_2))) (.bOverride_ColorGradingIntensity (Utilities|Struct|BreakPostProcessSettings (Variables|/Script/Engine.SceneCaptureComponent2D|GetPostProcessSettings _scenecapture2d1_2))) (.bOverride_ColorGradingLUT (Utilities|Struct|BreakPostProcessSettings (Variables|/Script/Engine.SceneCaptureComponent2D|GetPostProcessSettings _scenecapture2d1_2))) (.bOverride_DepthOfFieldFocalDistance (Utilities|Struct|BreakPostProcessSettings (Variables|/Script/Engine.SceneCaptureComponent2D|GetPostProcessSettings _scenecapture2d1_2))) (.bOverride_DepthOfFieldFocalRegion (Utilities|Struct|BreakPostProcessSettings (Variables|/Script/Engine.SceneCaptureComponent2D|GetPostProcessSettings _scenecapture2d1_2))) (.bOverride_DepthOfFieldNearTransitionRegion (Utilities|Struct|BreakPostProcessSettings (Variables|/Script/Engine.SceneCaptureComponent2D|GetPostProcessSettings _scenecapture2d1_2))) (.bOverride_DepthOfFieldFarTransitionRegion (Utilities|Struct|BreakPostProcessSettings (Variables|/Script/Engine.SceneCaptureComponent2D|GetPostProcessSettings _scenecapture2d1_2))) (.bOverride_DepthOfFieldScale (Utilities|Struct|BreakPostProcessSettings (Variables|/Script/Engine.SceneCaptureComponent2D|GetPostProcessSettings _scenecapture2d1_2))) (.bOverride_DepthOfFieldMaxBokehSize (Utilities|Struct|BreakPostProcessSettings (Variables|/Script/Engine.SceneCaptureComponent2D|GetPostProcessSettings _scenecapture2d1_2))) (.bOverride_DepthOfFieldNearBlurSize (Utilities|Struct|BreakPostProcessSettings (Variables|/Script/Engine.SceneCaptureComponent2D|GetPostProcessSettings _scenecapture2d1_2))) (.bOverride_DepthOfFieldFarBlurSize (Utilities|Struct|BreakPostProcessSettings (Variables|/Script/Engine.SceneCaptureComponent2D|GetPostProcessSettings _scenecapture2d1_2))) (.bOverride_DepthOfFieldMethod (Utilities|Struct|BreakPostProcessSettings (Variables|/Script/Engine.SceneCaptureComponent2D|GetPostProcessSettings _scenecapture2d1_2))) (.bOverride_DepthOfFieldBokehShape (Utilities|Struct|BreakPostProcessSettings (Variables|/Script/Engine.SceneCaptureComponent2D|GetPostProcessSettings _scenecapture2d1_2))) (.bOverride_DepthOfFieldOcclusion (Utilities|Struct|BreakPostProcessSettings (Variables|/Script/Engine.SceneCaptureComponent2D|GetPostProcessSettings _scenecapture2d1_2))) (.bOverride_DepthOfFieldColorThreshold (Utilities|Struct|BreakPostProcessSettings (Variables|/Script/Engine.SceneCaptureComponent2D|GetPostProcessSettings _scenecapture2d1_2))) (.bOverride_DepthOfFieldSizeThreshold (Utilities|Struct|BreakPostProcessSettings (Variables|/Script/Engine.SceneCaptureComponent2D|GetPostProcessSettings _scenecapture2d1_2))) (.bOverride_DepthOfFieldSkyFocusDistance (Utilities|Struct|BreakPostProcessSettings (Variables|/Script/Engine.SceneCaptureComponent2D|GetPostProcessSettings _scenecapture2d1_2))) (.bOverride_MotionBlurAmount (Utilities|Struct|BreakPostProcessSettings (Variables|/Script/Engine.SceneCaptureComponent2D|GetPostProcessSettings _scenecapture2d1_2))) (.bOverride_MotionBlurMax (Utilities|Struct|BreakPostProcessSettings (Variables|/Script/Engine.SceneCaptureComponent2D|GetPostProcessSettings _scenecapture2d1_2))) (.bOverride_MotionBlurPerObjectSize (Utilities|Struct|BreakPostProcessSettings (Variables|/Script/Engine.SceneCaptureComponent2D|GetPostProcessSettings _scenecapture2d1_2))) (.bOverride_ScreenPercentage (Utilities|Struct|BreakPostProcessSettings (Variables|/Script/Engine.SceneCaptureComponent2D|GetPostProcessSettings _scenecapture2d1_2))) (.bOverride_AntiAliasingMethod (Utilities|Struct|BreakPostProcessSettings (Variables|/Script/Engine.SceneCaptureComponent2D|GetPostProcessSettings _scenecapture2d1_2))) (.bOverride_ScreenSpaceReflectionIntensity (Utilities|Struct|BreakPostProcessSettings (Variables|/Script/Engine.SceneCaptureComponent2D|GetPostProcessSettings _scenecapture2d1_2))) (.bOverride_ScreenSpaceReflectionQuality (Utilities|Struct|BreakPostProcessSettings (Variables|/Script/Engine.SceneCaptureComponent2D|GetPostProcessSettings _scenecapture2d1_2))) (.bOverride_ScreenSpaceReflectionMaxRoughness (Utilities|Struct|BreakPostProcessSettings (Variables|/Script/Engine.SceneCaptureComponent2D|GetPostProcessSettings _scenecapture2d1_2))) (.bOverride_ScreenSpaceReflectionRoughnessScale (Utilities|Struct|BreakPostProcessSettings (Variables|/Script/Engine.SceneCaptureComponent2D|GetPostProcessSettings _scenecapture2d1_2))) (.FilmWhitePoint (Utilities|Struct|BreakPostProcessSettings (Variables|/Script/Engine.SceneCaptureComponent2D|GetPostProcessSettings _scenecapture2d1_2))) (.FilmShadowTint (Utilities|Struct|BreakPostProcessSettings (Variables|/Script/Engine.SceneCaptureComponent2D|GetPostProcessSettings _scenecapture2d1_2))) (.FilmShadowTintBlend (Utilities|Struct|BreakPostProcessSettings (Variables|/Script/Engine.SceneCaptureComponent2D|GetPostProcessSettings _scenecapture2d1_2))) (.FilmShadowTintAmount (Utilities|Struct|BreakPostProcessSettings (Variables|/Script/Engine.SceneCaptureComponent2D|GetPostProcessSettings _scenecapture2d1_2))) (Variables|Default|GetsaturationValue) (.FilmChannelMixerRed (Utilities|Struct|BreakPostProcessSettings (Variables|/Script/Engine.SceneCaptureComponent2D|GetPostProcessSettings _scenecapture2d1_2))) (.FilmChannelMixerGreen (Utilities|Struct|BreakPostProcessSettings (Variables|/Script/Engine.SceneCaptureComponent2D|GetPostProcessSettings _scenecapture2d1_2))) (.FilmChannelMixerBlue (Utilities|Struct|BreakPostProcessSettings (Variables|/Script/Engine.SceneCaptureComponent2D|GetPostProcessSettings _scenecapture2d1_2))) (.FilmContrast (Utilities|Struct|BreakPostProcessSettings (Variables|/Script/Engine.SceneCaptureComponent2D|GetPostProcessSettings _scenecapture2d1_2))) (.FilmToeAmount (Utilities|Struct|BreakPostProcessSettings (Variables|/Script/Engine.SceneCaptureComponent2D|GetPostProcessSettings _scenecapture2d1_2))) (.FilmHealAmount (Utilities|Struct|BreakPostProcessSettings (Variables|/Script/Engine.SceneCaptureComponent2D|GetPostProcessSettings _scenecapture2d1_2))) (.FilmDynamicRange (Utilities|Struct|BreakPostProcessSettings (Variables|/Script/Engine.SceneCaptureComponent2D|GetPostProcessSettings _scenecapture2d1_2))) (.SceneColorTint (Utilities|Struct|BreakPostProcessSettings (Variables|/Script/Engine.SceneCaptureComponent2D|GetPostProcessSettings _scenecapture2d1_2))) (.SceneFringeIntensity (Utilities|Struct|BreakPostProcessSettings (Variables|/Script/Engine.SceneCaptureComponent2D|GetPostProcessSettings _scenecapture2d1_2))) (.SceneFringeSaturation (Utilities|Struct|BreakPostProcessSettings (Variables|/Script/Engine.SceneCaptureComponent2D|GetPostProcessSettings _scenecapture2d1_2))) (.BloomIntensity (Utilities|Struct|BreakPostProcessSettings (Variables|/Script/Engine.SceneCaptureComponent2D|GetPostProcessSettings _scenecapture2d1_2))) (.BloomThreshold (Utilities|Struct|BreakPostProcessSettings (Variables|/Script/Engine.SceneCaptureComponent2D|GetPostProcessSettings _scenecapture2d1_2))) (.Bloom1Size (Utilities|Struct|BreakPostProcessSettings (Variables|/Script/Engine.SceneCaptureComponent2D|GetPostProcessSettings _scenecapture2d1_2))) (.Bloom2Size (Utilities|Struct|BreakPostProcessSettings (Variables|/Script/Engine.SceneCaptureComponent2D|GetPostProcessSettings _scenecapture2d1_2))) (.Bloom3Size (Utilities|Struct|BreakPostProcessSettings (Variables|/Script/Engine.SceneCaptureComponent2D|GetPostProcessSettings _scenecapture2d1_2))) (.Bloom4Size (Utilities|Struct|BreakPostProcessSettings (Variables|/Script/Engine.SceneCaptureComponent2D|GetPostProcessSettings _scenecapture2d1_2))) (.Bloom5Size (Utilities|Struct|BreakPostProcessSettings (Variables|/Script/Engine.SceneCaptureComponent2D|GetPostProcessSettings _scenecapture2d1_2))) (.Bloom1Tint (Utilities|Struct|BreakPostProcessSettings (Variables|/Script/Engine.SceneCaptureComponent2D|GetPostProcessSettings _scenecapture2d1_2))) (.Bloom2Tint (Utilities|Struct|BreakPostProcessSettings (Variables|/Script/Engine.SceneCaptureComponent2D|GetPostProcessSettings _scenecapture2d1_2))) (.Bloom3Tint (Utilities|Struct|BreakPostProcessSettings (Variables|/Script/Engine.SceneCaptureComponent2D|GetPostProcessSettings _scenecapture2d1_2))) (.Bloom4Tint (Utilities|Struct|BreakPostProcessSettings (Variables|/Script/Engine.SceneCaptureComponent2D|GetPostProcessSettings _scenecapture2d1_2))) (.Bloom5Tint (Utilities|Struct|BreakPostProcessSettings (Variables|/Script/Engine.SceneCaptureComponent2D|GetPostProcessSettings _scenecapture2d1_2))) (.BloomDirtMaskIntensity (Utilities|Struct|BreakPostProcessSettings (Variables|/Script/Engine.SceneCaptureComponent2D|GetPostProcessSettings _scenecapture2d1_2))) (.BloomDirtMaskTint (Utilities|Struct|BreakPostProcessSettings (Variables|/Script/Engine.SceneCaptureComponent2D|GetPostProcessSettings _scenecapture2d1_2))) (.BloomDirtMask (Utilities|Struct|BreakPostProcessSettings (Variables|/Script/Engine.SceneCaptureComponent2D|GetPostProcessSettings _scenecapture2d1_2))) (.LPVIntensity (Utilities|Struct|BreakPostProcessSettings (Variables|/Script/Engine.SceneCaptureComponent2D|GetPostProcessSettings _scenecapture2d1_2))) (.LPVWarpIntensity (Utilities|Struct|BreakPostProcessSettings (Variables|/Script/Engine.SceneCaptureComponent2D|GetPostProcessSettings _scenecapture2d1_2))) (.LPVVplInjectionBias (Utilities|Struct|BreakPostProcessSettings (Variables|/Script/Engine.SceneCaptureComponent2D|GetPostProcessSettings _scenecapture2d1_2))) (.LPVSize (Utilities|Struct|BreakPostProcessSettings (Variables|/Script/Engine.SceneCaptureComponent2D|GetPostProcessSettings _scenecapture2d1_2))) (.LPVSecondaryOcclusionIntensity (Utilities|Struct|BreakPostProcessSettings (Variables|/Script/Engine.SceneCaptureComponent2D|GetPostProcessSettings _scenecapture2d1_2))) (.LPVSecondaryBounceIntensity (Utilities|Struct|BreakPostProcessSettings (Variables|/Script/Engine.SceneCaptureComponent2D|GetPostProcessSettings _scenecapture2d1_2))) (.LPVGeometryVolumeBias (Utilities|Struct|BreakPostProcessSettings (Variables|/Script/Engine.SceneCaptureComponent2D|GetPostProcessSettings _scenecapture2d1_2))) (.LPVEmissiveInjectionIntensity (Utilities|Struct|BreakPostProcessSettings (Variables|/Script/Engine.SceneCaptureComponent2D|GetPostProcessSettings _scenecapture2d1_2))) (.LPVTransmissionIntensity (Utilities|Struct|BreakPostProcessSettings (Variables|/Script/Engine.SceneCaptureComponent2D|GetPostProcessSettings _scenecapture2d1_2))) (.AmbientCubemapTint (Utilities|Struct|BreakPostProcessSettings (Variables|/Script/Engine.SceneCaptureComponent2D|GetPostProcessSettings _scenecapture2d1_2))) (.AmbientCubemapIntensity (Utilities|Struct|BreakPostProcessSettings (Variables|/Script/Engine.SceneCaptureComponent2D|GetPostProcessSettings _scenecapture2d1_2))) (.AmbientCubemap (Utilities|Struct|BreakPostProcessSettings (Variables|/Script/Engine.SceneCaptureComponent2D|GetPostProcessSettings _scenecapture2d1_2))) (.AutoExposureLowPercent (Utilities|Struct|BreakPostProcessSettings (Variables|/Script/Engine.SceneCaptureComponent2D|GetPostProcessSettings _scenecapture2d1_2))) (.AutoExposureHighPercent (Utilities|Struct|BreakPostProcessSettings (Variables|/Script/Engine.SceneCaptureComponent2D|GetPostProcessSettings _scenecapture2d1_2))) (.AutoExposureMinBrightness (Utilities|Struct|BreakPostProcessSettings (Variables|/Script/Engine.SceneCaptureComponent2D|GetPostProcessSettings _scenecapture2d1_2))) (.AutoExposureMaxBrightness (Utilities|Struct|BreakPostProcessSettings (Variables|/Script/Engine.SceneCaptureComponent2D|GetPostProcessSettings _scenecapture2d1_2))) (.AutoExposureSpeedUp (Utilities|Struct|BreakPostProcessSettings (Variables|/Script/Engine.SceneCaptureComponent2D|GetPostProcessSettings _scenecapture2d1_2))) (.AutoExposureSpeedDown (Utilities|Struct|BreakPostProcessSettings (Variables|/Script/Engine.SceneCaptureComponent2D|GetPostProcessSettings _scenecapture2d1_2))) (.AutoExposureBias (Utilities|Struct|BreakPostProcessSettings (Variables|/Script/Engine.SceneCaptureComponent2D|GetPostProcessSettings _scenecapture2d1_2))) (.HistogramLogMin (Utilities|Struct|BreakPostProcessSettings (Variables|/Script/Engine.SceneCaptureComponent2D|GetPostProcessSettings _scenecapture2d1_2))) (.HistogramLogMax (Utilities|Struct|BreakPostProcessSettings (Variables|/Script/Engine.SceneCaptureComponent2D|GetPostProcessSettings _scenecapture2d1_2))) (.LensFlareIntensity (Utilities|Struct|BreakPostProcessSettings (Variables|/Script/Engine.SceneCaptureComponent2D|GetPostProcessSettings _scenecapture2d1_2))) (.LensFlareTint (Utilities|Struct|BreakPostProcessSettings (Variables|/Script/Engine.SceneCaptureComponent2D|GetPostProcessSettings _scenecapture2d1_2))) (.LensFlareBokehSize (Utilities|Struct|BreakPostProcessSettings (Variables|/Script/Engine.SceneCaptureComponent2D|GetPostProcessSettings _scenecapture2d1_2))) (.LensFlareThreshold (Utilities|Struct|BreakPostProcessSettings (Variables|/Script/Engine.SceneCaptureComponent2D|GetPostProcessSettings _scenecapture2d1_2))) (.LensFlareBokehShape (Utilities|Struct|BreakPostProcessSettings (Variables|/Script/Engine.SceneCaptureComponent2D|GetPostProcessSettings _scenecapture2d1_2))) (.VignetteIntensity (Utilities|Struct|BreakPostProcessSettings (Variables|/Script/Engine.SceneCaptureComponent2D|GetPostProcessSettings _scenecapture2d1_2))) (.VignetteColor (Utilities|Struct|BreakPostProcessSettings (Variables|/Script/Engine.SceneCaptureComponent2D|GetPostProcessSettings _scenecapture2d1_2))) (.GrainJitter (Utilities|Struct|BreakPostProcessSettings (Variables|/Script/Engine.SceneCaptureComponent2D|GetPostProcessSettings _scenecapture2d1_2))) (.GrainIntensity (Utilities|Struct|BreakPostProcessSettings (Variables|/Script/Engine.SceneCaptureComponent2D|GetPostProcessSettings _scenecapture2d1_2))) (.AmbientOcclusionIntensity (Utilities|Struct|BreakPostProcessSettings (Variables|/Script/Engine.SceneCaptureComponent2D|GetPostProcessSettings _scenecapture2d1_2))) (.AmbientOcclusionStaticFraction (Utilities|Struct|BreakPostProcessSettings (Variables|/Script/Engine.SceneCaptureComponent2D|GetPostProcessSettings _scenecapture2d1_2))) (.AmbientOcclusionRadius (Utilities|Struct|BreakPostProcessSettings (Variables|/Script/Engine.SceneCaptureComponent2D|GetPostProcessSettings _scenecapture2d1_2))) (.AmbientOcclusionRadiusInWS (Utilities|Struct|BreakPostProcessSettings (Variables|/Script/Engine.SceneCaptureComponent2D|GetPostProcessSettings _scenecapture2d1_2))) (.AmbientOcclusionFadeDistance (Utilities|Struct|BreakPostProcessSettings (Variables|/Script/Engine.SceneCaptureComponent2D|GetPostProcessSettings _scenecapture2d1_2))) (.AmbientOcclusionFadeRadius (Utilities|Struct|BreakPostProcessSettings (Variables|/Script/Engine.SceneCaptureComponent2D|GetPostProcessSettings _scenecapture2d1_2))) (.AmbientOcclusionDistance (Utilities|Struct|BreakPostProcessSettings (Variables|/Script/Engine.SceneCaptureComponent2D|GetPostProcessSettings _scenecapture2d1_2))) (.AmbientOcclusionPower (Utilities|Struct|BreakPostProcessSettings (Variables|/Script/Engine.SceneCaptureComponent2D|GetPostProcessSettings _scenecapture2d1_2))) (.AmbientOcclusionBias (Utilities|Struct|BreakPostProcessSettings (Variables|/Script/Engine.SceneCaptureComponent2D|GetPostProcessSettings _scenecapture2d1_2))) (.AmbientOcclusionQuality (Utilities|Struct|BreakPostProcessSettings (Variables|/Script/Engine.SceneCaptureComponent2D|GetPostProcessSettings _scenecapture2d1_2))) (.AmbientOcclusionMipBlend (Utilities|Struct|BreakPostProcessSettings (Variables|/Script/Engine.SceneCaptureComponent2D|GetPostProcessSettings _scenecapture2d1_2))) (.AmbientOcclusionMipScale (Utilities|Struct|BreakPostProcessSettings (Variables|/Script/Engine.SceneCaptureComponent2D|GetPostProcessSettings _scenecapture2d1_2))) (.AmbientOcclusionMipThreshold (Utilities|Struct|BreakPostProcessSettings (Variables|/Script/Engine.SceneCaptureComponent2D|GetPostProcessSettings _scenecapture2d1_2))) (.IndirectLightingColor (Utilities|Struct|BreakPostProcessSettings (Variables|/Script/Engine.SceneCaptureComponent2D|GetPostProcessSettings _scenecapture2d1_2))) (.IndirectLightingIntensity (Utilities|Struct|BreakPostProcessSettings (Variables|/Script/Engine.SceneCaptureComponent2D|GetPostProcessSettings _scenecapture2d1_2))) (.ColorGradingIntensity (Utilities|Struct|BreakPostProcessSettings (Variables|/Script/Engine.SceneCaptureComponent2D|GetPostProcessSettings _scenecapture2d1_2))) (.ColorGradingLUT (Utilities|Struct|BreakPostProcessSettings (Variables|/Script/Engine.SceneCaptureComponent2D|GetPostProcessSettings _scenecapture2d1_2))) (.DepthOfFieldMethod (Utilities|Struct|BreakPostProcessSettings (Variables|/Script/Engine.SceneCaptureComponent2D|GetPostProcessSettings _scenecapture2d1_2))) (.DepthOfFieldFocalDistance (Utilities|Struct|BreakPostProcessSettings (Variables|/Script/Engine.SceneCaptureComponent2D|GetPostProcessSettings _scenecapture2d1_2))) (.DepthOfFieldFocalRegion (Utilities|Struct|BreakPostProcessSettings (Variables|/Script/Engine.SceneCaptureComponent2D|GetPostProcessSettings _scenecapture2d1_2))) (.DepthOfFieldNearTransitionRegion (Utilities|Struct|BreakPostProcessSettings (Variables|/Script/Engine.SceneCaptureComponent2D|GetPostProcessSettings _scenecapture2d1_2))) (.DepthOfFieldFarTransitionRegion (Utilities|Struct|BreakPostProcessSettings (Variables|/Script/Engine.SceneCaptureComponent2D|GetPostProcessSettings _scenecapture2d1_2))) (.DepthOfFieldScale (Utilities|Struct|BreakPostProcessSettings (Variables|/Script/Engine.SceneCaptureComponent2D|GetPostProcessSettings _scenecapture2d1_2))) (.DepthOfFieldMaxBokehSize (Utilities|Struct|BreakPostProcessSettings (Variables|/Script/Engine.SceneCaptureComponent2D|GetPostProcessSettings _scenecapture2d1_2))) (.DepthOfFieldNearBlurSize (Utilities|Struct|BreakPostProcessSettings (Variables|/Script/Engine.SceneCaptureComponent2D|GetPostProcessSettings _scenecapture2d1_2))) (.DepthOfFieldFarBlurSize (Utilities|Struct|BreakPostProcessSettings (Variables|/Script/Engine.SceneCaptureComponent2D|GetPostProcessSettings _scenecapture2d1_2))) (.DepthOfFieldBokehShape (Utilities|Struct|BreakPostProcessSettings (Variables|/Script/Engine.SceneCaptureComponent2D|GetPostProcessSettings _scenecapture2d1_2))) (.DepthOfFieldOcclusion (Utilities|Struct|BreakPostProcessSettings (Variables|/Script/Engine.SceneCaptureComponent2D|GetPostProcessSettings _scenecapture2d1_2))) (.DepthOfFieldColorThreshold (Utilities|Struct|BreakPostProcessSettings (Variables|/Script/Engine.SceneCaptureComponent2D|GetPostProcessSettings _scenecapture2d1_2))) (.DepthOfFieldSizeThreshold (Utilities|Struct|BreakPostProcessSettings (Variables|/Script/Engine.SceneCaptureComponent2D|GetPostProcessSettings _scenecapture2d1_2))) (.DepthOfFieldSkyFocusDistance (Utilities|Struct|BreakPostProcessSettings (Variables|/Script/Engine.SceneCaptureComponent2D|GetPostProcessSettings _scenecapture2d1_2))) (.MotionBlurAmount (Utilities|Struct|BreakPostProcessSettings (Variables|/Script/Engine.SceneCaptureComponent2D|GetPostProcessSettings _scenecapture2d1_2))) (.MotionBlurMax (Utilities|Struct|BreakPostProcessSettings (Variables|/Script/Engine.SceneCaptureComponent2D|GetPostProcessSettings _scenecapture2d1_2))) (.MotionBlurPerObjectSize (Utilities|Struct|BreakPostProcessSettings (Variables|/Script/Engine.SceneCaptureComponent2D|GetPostProcessSettings _scenecapture2d1_2))) (.ScreenPercentage (Utilities|Struct|BreakPostProcessSettings (Variables|/Script/Engine.SceneCaptureComponent2D|GetPostProcessSettings _scenecapture2d1_2))) (.AntiAliasingMethod (Utilities|Struct|BreakPostProcessSettings (Variables|/Script/Engine.SceneCaptureComponent2D|GetPostProcessSettings _scenecapture2d1_2))) (.ScreenSpaceReflectionIntensity (Utilities|Struct|BreakPostProcessSettings (Variables|/Script/Engine.SceneCaptureComponent2D|GetPostProcessSettings _scenecapture2d1_2))) (.ScreenSpaceReflectionQuality (Utilities|Struct|BreakPostProcessSettings (Variables|/Script/Engine.SceneCaptureComponent2D|GetPostProcessSettings _scenecapture2d1_2))) (.ScreenSpaceReflectionMaxRoughness (Utilities|Struct|BreakPostProcessSettings (Variables|/Script/Engine.SceneCaptureComponent2D|GetPostProcessSettings _scenecapture2d1_2))) (.Blendables (Utilities|Struct|BreakPostProcessSettings (Variables|/Script/Engine.SceneCaptureComponent2D|GetPostProcessSettings _scenecapture2d1_2))))))
    (elif (Variables|Default|GetmemoryTriggered)
      ;[1 1 1] Delay a bit and then zoom in
      (if true
        (if (> (Variables|/Script/Engine.SceneCaptureComponent2D|GetFOVAngle _scenecapture2d1) 5e+01)
          (Variables|/Script/Engine.SceneCaptureComponent2D|SetFOVAngle _scenecapture2d1 (- (Variables|/Script/Engine.SceneCaptureComponent2D|GetFOVAngle _scenecapture2d1) 0.1)))
        (else
          (Variables|Default|Setcounter (- (Variables|Default|Getcounter) 1)))))))

(fn ConstructionScript)