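; Blueprint for a roadside-scene memory sequence that moves and turns a camera when the player triggers the sign.
; While MemoryTriggered is set, Tick nudges Camera1 by a fixed world offset and decrements Counter, then sets MemoryFinished at zero.
; A separate Yaw countdown limits how many of those steps also rotate the camera.
; Motion is stepped per frame without delta time, so its speed depends on frame rate.
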(event EventTick
  (params (DeltaSeconds :type Float%20%28single-precision%29))
  (bind _camera1 (Variables|Default|GetCamera1))
  (bind _returnvalue (Transformation|GetWorldLocation _camera1))
  (bind _returnvalue_2 (Transformation|GetWorldRotation _camera1))
  (bind (_x _y _z) (Math|Vector|BreakVector _returnvalue))
  (bind (_pitch _yaw _roll) (Class|KismetMathLibrary|BreakRot _returnvalue_2))
  ;[1 1 1] When the player triggers the sign, camera rotates
  (if (Variables|Default|GetmemoryTriggered)
    (if (== (Variables|Default|Getcounter) 0)
      (Variables|Default|SetmemoryFinished true)
      (else
        (Transformation|SetWorldLocation _camera1 (Math|Vector|MakeVector (+ _x 0.8) (- _y 0.8) (+ _z 0.1)) false)
        (Variables|Default|Setcounter (- (Variables|Default|Getcounter) 1))
        (if (not (== (Variables|Default|Getyaw) 0))
          (Transformation|SetWorldRotation _camera1 (Class|KismetMathLibrary|MakeRot _pitch (- _yaw 1.0) _roll) false)
          (Variables|Default|Setyaw (- (Variables|Default|Getyaw) 1)))))))

(fn ConstructionScript)