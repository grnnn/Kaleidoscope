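; Roadside-scene camera Blueprint that fades scene-capture saturation and pans its camera for a sign-triggered memory moment.
; While ChangeSat is set, Tick raises SaturationValue toward 0.5 and rebuilds SceneCapture2D1's post-process settings with it.
; While MemoryTriggered is set, Tick yaws Camera1 in small steps until Counter runs out.
; The pan runs only while ChangeSat is off or saturation is still below the cap.
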(event EventTick
  (params (DeltaSeconds :type Float%20%28single-precision%29))
  (bind _camera1 (Variables|Default|GetCamera1))
  (bind _scenecapture2d1 (Variables|Default|GetSceneCapture2D1))
  (bind _returnvalue (Transformation|GetWorldRotation _camera1))
  (bind (_pitch _yaw _roll) (Class|KismetMathLibrary|BreakRot _returnvalue))
  ;[1 1 1] When the player triggers the sign, camera rotates
  ;[1 1 1] Saturation Change
  (if (Variables|Default|GetChangeSat)
    (if (< (Variables|Default|GetsaturationValue) 0.5)
      (Variables|Default|SetsaturationValue (- (Variables|Default|GetsaturationValue) -0.005))
      (Variables|/Script/Engine.SceneCaptureComponent2D|SetPostProcessSettings _scenecapture2d1 (Utilities|Struct|MakePostProcessSettings (.bOverride_FilmWhitePoint (Utilities|Struct|BreakPostProcessSettings (Variables|/Script/Engine.SceneCaptureComponent2D|GetPostProcessSettings _scenecapture2d1))) true (.bOverride_FilmChannelMixerRed (Utilities|Struct|BreakPostProcessSettings (Variables|/Script/Engine.SceneCaptureComponent2D|GetPostProcessSettings _scenecapture2d1))) (.bOverride_FilmChannelMixerGreen (Utilities|Struct|BreakPostProcessSettings (Variables|/Script/Engine.SceneCaptureComponent2D|GetPostProcessSettings _scenecapture2d1))) (.bOverride_FilmChannelMixerBlue (Utilities|Struct|BreakPostProcessSettings (Variables|/Script/Engine.SceneCaptureComponent2D|GetPostProcessSettings _scenecapture2d1))) (.bOverride_FilmContrast (Utilities|Struct|BreakPostProcessSettings (Variables|/Script/Engine.SceneCaptureComponent2D|GetPostProcessSettings _scenecapture2d1))) (.bOverride_FilmDynamicRange (Utilities|Struct|BreakPostProcessSettings (Variables|/Script/Engine.SceneCaptureComponent2D|GetPostProcessSettings _scenecapture2d1))) (.bOverride_FilmHealAmount (Utilities|Struct|BreakPostProcessSettings (Variables|/Script/Engine.SceneCaptureComponent2D|GetPostProcessSettings _scenecapture2d1))) (.bOverride_FilmToeAmount (Utilities|Struct|BreakPostProcessSettings (Variables|/Script/Engine.SceneCaptureComponent2D|GetPostProcessSettings _scenecapture2d1))) (.bOverride_FilmShadowTint (Utilities|Struct|BreakPostProcessSettings (Variables|/Script/Engine.SceneCaptureComponent2D|GetPostProcessSettings _scenecapture2d1))) (.bOverride_FilmShadowTintBlend (Utilities|Struct|BreakPostProcessSettings (Variables|/Script/Engine.SceneCaptureComponent2D|GetPostProcessSettings _scenecapture2d1))) (.bOverride_FilmShadowTintAmount (Utilities|Struct|BreakPostProcessSettings (Variables|/Script/Engine.SceneCaptureComponent2D|GetPostProcessSettings _scenecapture2d1))) (.bOverride_SceneColorTint (Utilities|Struct|BreakPostProcessSettings (Variables|/Script/Engine.SceneCaptureComponent2D|GetPostProcessSettings _scenecapture2d1))) (.bOverride_SceneFringeIntensity (Utilities|Struct|BreakPostProcessSettings (Variables|/Script/Engine.SceneCaptureComponent2D|GetPostProcessSettings _scenecapture2d1))) (.bOverride_SceneFringeSaturation (Utilities|Struct|BreakPostProcessSettings (Variables|/Script/Engine.SceneCaptureComponent2D|GetPostProcessSettings _scenecapture2d1))) (.bOverride_AmbientCubemapTint (Utilities|Struct|BreakPostProcessSettings (Variables|/Script/Engine.SceneCaptureComponent2D|GetPostProcessSettings _scenecapture2d1))) (.bOverride_AmbientCubemapIntensity (Utilities|Struct|BreakPostProcessSettings (Variables|/Script/Engine.SceneCaptureComponent2D|GetPostProcessSettings _scenecapture2d1))) (.bOverride_BloomIntensity (Utilities|Struct|BreakPostProcessSettings (Variables|/Script/Engine.SceneCaptureComponent2D|GetPostProcessSettings _scenecapture2d1))) (.bOverride_BloomThreshold (Utilities|Struct|BreakPostProcessSettings (Variables|/Script/Engine.SceneCaptureComponent2D|GetPostProcessSettings _scenecapture2d1))) (.bOverride_Bloom1Tint (Utilities|Struct|BreakPostProcessSettings (Variables|/Script/Engine.SceneCaptureComponent2D|GetPostProcessSettings _scenecapture2d1))) (.bOverride_Bloom1Size (Utilities|Struct|BreakPostProcessSettings (Variables|/Script/Engine.SceneCaptureComponent2D|GetPostProcessSettings _scenecapture2d1))) (.bOverride_Bloom2Size (Utilities|Struct|BreakPostProcessSettings (Variables|/Script/Engine.SceneCaptureComponent2D|GetPostProcessSettings _scenecapture2d1))) (.bOverride_Bloom2Tint (Utilities|Struct|BreakPostProcessSettings (Variables|/Script/Engine.SceneCaptureComponent2D|GetPostProcessSettings _scenecapture2d1))) (.bOverride_Bloom3Tint (Utilities|Struct|BreakPostProcessSettings (Variables|/Script/Engine.SceneCaptureComponent2D|GetPostProcessSettings _scenecapture2d1))) (.bOverride_Bloom3Size (Utilities|Struct|BreakPostProcessSettings (Variables|/Script/Engine.SceneCaptureComponent2D|GetPostProcessSettings _scenecapture2d1))) (.bOverride_Bloom4Tint (Utilities|Struct|BreakPostProcessSettings (Variables|/Script/Engine.SceneCaptureComponent2D|GetPostProcessSettings _scenecapture2d1))) (.bOverride_Bloom4Size (Utilities|Struct|BreakPostProcessSettings (Variables|/Script/Engine.SceneCaptureComponent2D|GetPostProcessSettings _scenecapture2d1))) (.bOverride_Bloom5Tint (Utilities|Struct|BreakPostProcessSettings (Variables|/Script/Engine.SceneCaptureComponent2D|GetPostProcessSettings _scenecapture2d1))) (.bOverride_Bloom5Size (Utilities|Struct|BreakPostProcessSettings (Variables|/Script/Engine.SceneCaptureComponent2D|GetPostProcessSettings _scenecapture2d1))) (.bOverride_BloomDirtMaskIntensity (Utilities|Struct|BreakPostProcessSettings (Variables|/Script/Engine.SceneCaptureComponent2D|GetPostProcessSettings _scenecapture2d1))) (.bOverride_BloomDirtMaskTint (Utilities|Struct|BreakPostProcessSettings (Variables|/Script/Engine.SceneCaptureComponent2D|GetPostProcessSettings _scenecapture2d1))) (.bOverride_BloomDirtMask (Utilities|Struct|BreakPostProcessSettings (Variables|/Script/Engine.SceneCaptureComponent2D|GetPostProcessSettings _scenecapture2d1))) (.bOverride_AutoExposureLowPercent (Utilities|Struct|BreakPostProcessSettings (Variables|/Script/Engine.SceneCaptureComponent2D|GetPostProcessSettings _scenecapture2d1))) (.bOverride_AutoExposureHighPercent (Utilities|Struct|BreakPostProcessSettings (Variables|/Script/Engine.SceneCaptureComponent2D|GetPostProcessSettings _scenecapture2d1))) (.bOverride_AutoExposureMinBrightness (Utilities|Struct|BreakPostProcessSettings (Variables|/Script/Engine.SceneCaptureComponent2D|GetPostProcessSettings _scenecapture2d1))) (.bOverride_AutoExposureMaxBrightness (Utilities|Struct|BreakPostProcessSettings (Variables|/Script/Engine.SceneCaptureComponent2D|GetPostProcessSettings _scenecapture2d1))) (.bOverride_AutoExposureSpeedUp (Utilities|Struct|BreakPostProcessSettings (Variables|/Script/Engine.SceneCaptureComponent2D|GetPostProcessSettings _scenecapture2d1))) (.bOverride_AutoExposureSpeedDown (Utilities|Struct|BreakPostProcessSettings (Variables|/Script/Engine.SceneCaptureComponent2D|GetPostProcessSettings _scenecapture2d1))) (.bOverride_AutoExposureBias (Utilities|Struct|BreakPostProcessSettings (Variables|/Script/Engine.SceneCaptureComponent2D|GetPostProcessSettings _scenecapture2d1))) (.bOverride_HistogramLogMin (Utilities|Struct|BreakPostProcessSettings (Variables|/Script/Engine.SceneCaptureComponent2D|GetPostProcessSettings _scenecapture2d1))) (.bOverride_HistogramLogMax (Utilities|Struct|BreakPostProcessSettings (Variables|/Script/Engine.SceneCaptureComponent2D|GetPostProcessSettings _scenecapture2d1))) (.bOverride_LensFlareIntensity (Utilities|Struct|BreakPostProcessSettings (Variables|/Script/Engine.SceneCaptureComponent2D|GetPostProcessSettings _scenecapture2d1))) (.bOverride_LensFlareTint (Utilities|Struct|BreakPostProcessSettings (Variables|/Script/Engine.SceneCaptureComponent2D|GetPostProcessSettings _scenecapture2d1))) (.bOverride_LensFlareTints (Utilities|Struct|BreakPostProcessSettings (Variables|/Script/Engine.SceneCaptureComponent2D|GetPostProcessSettings _scenecapture2d1))) (.bOverride_LensFlareBokehSize (Utilities|Struct|BreakPostProcessSettings (Variables|/Script/Engine.SceneCaptureComponent2D|GetPostProcessSettings _scenecapture2d1))) (.bOverride_LensFlareBokehShape (Utilities|Struct|BreakPostProcessSettings (Variables|/Script/Engine.SceneCaptureComponent2D|GetPostProcessSettings _scenecapture2d1))) (.bOverride_LensFlareThreshold (Utilities|Struct|BreakPostProcessSettings (Variables|/Script/Engine.SceneCaptureComponent2D|GetPostProcessSettings _scenecapture2d1))) (.bOverride_VignetteIntensity (Utilities|Struct|BreakPostProcessSettings (Variables|/Script/Engine.SceneCaptureComponent2D|GetPostProcessSettings _scenecapture2d1))) (.bOverride_VignetteColor (Utilities|Struct|BreakPostProcessSettings (Variables|/Script/Engine.SceneCaptureComponent2D|GetPostProcessSettings _scenecapture2d1))) (.bOverride_GrainIntensity (Utilities|Struct|BreakPostProcessSettings (Variables|/Script/Engine.SceneCaptureComponent2D|GetPostProcessSettings _scenecapture2d1))) (.bOverride_GrainJitter (Utilities|Struct|BreakPostProcessSettings (Variables|/Script/Engine.SceneCaptureComponent2D|GetPostProcessSettings _scenecapture2d1))) (.bOverride_AmbientOcclusionIntensity (Utilities|Struct|BreakPostProcessSettings (Variables|/Script/Engine.SceneCaptureComponent2D|GetPostProcessSettings _scenecapture2d1))) (.bOverride_AmbientOcclusionStaticFraction (Utilities|Struct|BreakPostProcessSettings (Variables|/Script/Engine.SceneCaptureComponent2D|GetPostProcessSettings _scenecapture2d1))) (.bOverride_AmbientOcclusionRadius (Utilities|Struct|BreakPostProcessSettings (Variables|/Script/Engine.SceneCaptureComponent2D|GetPostProcessSettings _scenecapture2d1))) (.bOverride_AmbientOcclusionFadeDistance (Utilities|Struct|BreakPostProcessSettings (Variables|/Script/Engine.SceneCaptureComponent2D|GetPostProcessSettings _scenecapture2d1))) (.bOverride_AmbientOcclusionFadeRadius (Utilities|Struct|BreakPostProcessSettings (Variables|/Script/Engine.SceneCaptureComponent2D|GetPostProcessSettings _scenecapture2d1))) (.bOverride_AmbientOcclusionDistance (Utilities|Struct|BreakPostProcessSettings (Variables|/Script/Engine.SceneCaptureComponent2D|GetPostProcessSettings _scenecapture2d1))) (.bOverride_AmbientOcclusionRadiusInWS (Utilities|Struct|BreakPostProcessSettings (Variables|/Script/Engine.SceneCaptureComponent2D|GetPostProcessSettings _scenecapture2d1))) (.bOverride_AmbientOcclusionPower (Utilities|Struct|BreakPostProcessSettings (Variables|/Script/Engine.SceneCaptureComponent2D|GetPostProcessSettings _scenecapture2d1))) (.bOverride_AmbientOcclusionBias (Utilities|Struct|BreakPostProcessSettings (Variables|/Script/Engine.SceneCaptureComponent2D|GetPostProcessSettings _scenecapture2d1))) (.bOverride_AmbientOcclusionQuality (Utilities|Struct|BreakPostProcessSettings (Variables|/Script/Engine.SceneCaptureComponent2D|GetPostProcessSettings _scenecapture2d1))) (.bOverride_AmbientOcclusionMipBlend (Utilities|Struct|BreakPostProcessSettings (Variables|/Script/Engine.SceneCaptureComponent2D|GetPostProcessSettings _scenecapture2d1))) (.bOverride_AmbientOcclusionMipScale (Utilities|Struct|BreakPostProcessSettings (Variables|/Script/Engine.SceneCaptureComponent2D|GetPostProcessSettings _scenecapture2d1))) (.bOverride_AmbientOcclusionMipThreshold (Utilities|Struct|BreakPostProcessSettings (Variables|/Script/Engine.SceneCaptureComponent2D|GetPostProcessSettings _scenecapture2d1))) (.bOverride_LPVIntensity (Utilities|Struct|BreakPostProcessSettings (Variables|/Script/Engine.SceneCaptureComponent2D|GetPostProcessSettings _scenecapture2d1))) (.bOverride_LPVWarpIntensity (Utilities|Struct|BreakPostProcessSettings (Variables|/Script/Engine.SceneCaptureComponent2D|GetPostProcessSettings _scenecapture2d1))) (.bOverride_LPVSize (Utilities|Struct|BreakPostProcessSettings (Variables|/Script/Engine.SceneCaptureComponent2D|GetPostProcessSettings _scenecapture2d1))) (.bOverride_LPVSecondaryOcclusionIntensity (Utilities|Struct|BreakPostProcessSettings (Variables|/Script/Engine.SceneCaptureComponent2D|GetPostProcessSettings _scenecapture2d1))) (.bOverride_LPVSecondaryBounceIntensity (Utilities|Struct|BreakPostProcessSettings (Variables|/Script/Engine.SceneCaptureComponent2D|GetPostProcessSettings _scenecapture2d1))) (.bOverride_LPVGeometryVolumeBias (Utilities|Struct|BreakPostProcessSettings (Variables|/Script/Engine.SceneCaptureComponent2D|GetPostProcessSettings _scenecapture2d1))) (.bOverride_LPVVplInjectionBias (Utilities|Struct|BreakPostProcessSettings (Variables|/Script/Engine.SceneCaptureComponent2D|GetPostProcessSettings _scenecapture2d1))) (.bOverride_LPVEmissiveInjectionIntensity (Utilities|Struct|BreakPostProcessSettings (Variables|/Script/Engine.SceneCaptureComponent2D|GetPostProcessSettings _scenecapture2d1))) (.bOverride_LPVTransmissionIntensity (Utilities|Struct|BreakPostProcessSettings (Variables|/Script/Engine.SceneCaptureComponent2D|GetPostProcessSettings _scenecapture2d1))) (.bOverride_IndirectLightingColor (Utilities|Struct|BreakPostProcessSettings (Variables|/Script/Engine.SceneCaptureComponent2D|GetPostProcessSettings _scenecapture2d1))) (.bOverride_IndirectLightingIntensity (Utilities|Struct|BreakPostProcessSettings (Variables|/Script/Engine.SceneCaptureComponent2D|GetPostProcessSettings _scenecapture2d1))) (.bOverride_ColorGradingIntensity (Utilities|Struct|BreakPostProcessSettings (Variables|/Script/Engine.SceneCaptureComponent2D|GetPostProcessSettings _scenecapture2d1))) (.bOverride_ColorGradingLUT (Utilities|Struct|BreakPostProcessSettings (Variables|/Script/Engine.SceneCaptureComponent2D|GetPostProcessSettings _scenecapture2d1))) (.bOverride_DepthOfFieldFocalDistance (Utilities|Struct|BreakPostProcessSettings (Variables|/Script/Engine.SceneCaptureComponent2D|GetPostProcessSettings _scenecapture2d1))) (.bOverride_DepthOfFieldFocalRegion (Utilities|Struct|BreakPostProcessSettings (Variables|/Script/Engine.SceneCaptureComponent2D|GetPostProcessSettings _scenecapture2d1))) (.bOverride_DepthOfFieldNearTransitionRegion (Utilities|Struct|BreakPostProcessSettings (Variables|/Script/Engine.SceneCaptureComponent2D|GetPostProcessSettings _scenecapture2d1))) (.bOverride_DepthOfFieldFarTransitionRegion (Utilities|Struct|BreakPostProcessSettings (Variables|/Script/Engine.SceneCaptureComponent2D|GetPostProcessSettings _scenecapture2d1))) (.bOverride_DepthOfFieldScale (Utilities|Struct|BreakPostProcessSettings (Variables|/Script/Engine.SceneCaptureComponent2D|GetPostProcessSettings _scenecapture2d1))) (.bOverride_DepthOfFieldMaxBokehSize (Utilities|Struct|BreakPostProcessSettings (Variables|/Script/Engine.SceneCaptureComponent2D|GetPostProcessSettings _scenecapture2d1))) (.bOverride_DepthOfFieldNearBlurSize (Utilities|Struct|BreakPostProcessSettings (Variables|/Script/Engine.SceneCaptureComponent2D|GetPostProcessSettings _scenecapture2d1))) (.bOverride_DepthOfFieldFarBlurSize (Utilities|Struct|BreakPostProcessSettings (Variables|/Script/Engine.SceneCaptureComponent2D|GetPostProcessSettings _scenecapture2d1))) (.bOverride_DepthOfFieldMethod (Utilities|Struct|BreakPostProcessSettings (Variables|/Script/Engine.SceneCaptureComponent2D|GetPostProcessSettings _scenecapture2d1))) (.bOverride_DepthOfFieldBokehShape (Utilities|Struct|BreakPostProcessSettings (Variables|/Script/Engine.SceneCaptureComponent2D|GetPostProcessSettings _scenecapture2d1))) (.bOverride_DepthOfFieldOcclusion (Utilities|Struct|BreakPostProcessSettings (Variables|/Script/Engine.SceneCaptureComponent2D|GetPostProcessSettings _scenecapture2d1))) (.bOverride_DepthOfFieldColorThreshold (Utilities|Struct|BreakPostProcessSettings (Variables|/Script/Engine.SceneCaptureComponent2D|GetPostProcessSettings _scenecapture2d1))) (.bOverride_DepthOfFieldSizeThreshold (Utilities|Struct|BreakPostProcessSettings (Variables|/Script/Engine.SceneCaptureComponent2D|GetPostProcessSettings _scenecapture2d1))) (.bOverride_DepthOfFieldSkyFocusDistance (Utilities|Struct|BreakPostProcessSettings (Variables|/Script/Engine.SceneCaptureComponent2D|GetPostProcessSettings _scenecapture2d1))) (.bOverride_MotionBlurAmount (Utilities|Struct|BreakPostProcessSettings (Variables|/Script/Engine.SceneCaptureComponent2D|GetPostProcessSettings _scenecapture2d1))) (.bOverride_MotionBlurMax (Utilities|Struct|BreakPostProcessSettings (Variables|/Script/Engine.SceneCaptureComponent2D|GetPostProcessSettings _scenecapture2d1))) (.bOverride_MotionBlurPerObjectSize (Utilities|Struct|BreakPostProcessSettings (Variables|/Script/Engine.SceneCaptureComponent2D|GetPostProcessSettings _scenecapture2d1))) (.bOverride_ScreenPercentage (Utilities|Struct|BreakPostProcessSettings (Variables|/Script/Engine.SceneCaptureComponent2D|GetPostProcessSettings _scenecapture2d1))) (.bOverride_AntiAliasingMethod (Utilities|Struct|BreakPostProcessSettings (Variables|/Script/Engine.SceneCaptureComponent2D|GetPostProcessSettings _scenecapture2d1))) (.bOverride_ScreenSpaceReflectionIntensity (Utilities|Struct|BreakPostProcessSettings (Variables|/Script/Engine.SceneCaptureComponent2D|GetPostProcessSettings _scenecapture2d1))) (.bOverride_ScreenSpaceReflectionQuality (Utilities|Struct|BreakPostProcessSettings (Variables|/Script/Engine.SceneCaptureComponent2D|GetPostProcessSettings _scenecapture2d1))) (.bOverride_ScreenSpaceReflectionMaxRoughness (Utilities|Struct|BreakPostProcessSettings (Variables|/Script/Engine.SceneCaptureComponent2D|GetPostProcessSettings _scenecapture2d1))) (.bOverride_ScreenSpaceReflectionRoughnessScale (Utilities|Struct|BreakPostProcessSettings (Variables|/Script/Engine.SceneCaptureComponent2D|GetPostProcessSettings _scenecapture2d1))) (.FilmWhitePoint (Utilities|Struct|BreakPostProcessSettings (Variables|/Script/Engine.SceneCaptureComponent2D|GetPostProcessSettings _scenecapture2d1))) (.FilmShadowTint (Utilities|Struct|BreakPostProcessSettings (Variables|/Script/Engine.SceneCaptureComponent2D|GetPostProcessSettings _scenecapture2d1))) (.FilmShadowTintBlend (Utilities|Struct|BreakPostProcessSettings (Variables|/Script/Engine.SceneCaptureComponent2D|GetPostProcessSettings _scenecapture2d1))) (.FilmShadowTintAmount (Utilities|Struct|BreakPostProcessSettings (Variables|/Script/Engine.SceneCaptureComponent2D|GetPostProcessSettings _scenecapture2d1))) (Variables|Default|GetsaturationValue) (.FilmChannelMixerRed (Utilities|Struct|BreakPostProcessSettings (Variables|/Script/Engine.SceneCaptureComponent2D|GetPostProcessSettings _scenecapture2d1))) (.FilmChannelMixerGreen (Utilities|Struct|BreakPostProcessSettings (Variables|/Script/Engine.SceneCaptureComponent2D|GetPostProcessSettings _scenecapture2d1))) (.FilmChannelMixerBlue (Utilities|Struct|BreakPostProcessSettings (Variables|/Script/Engine.SceneCaptureComponent2D|GetPostProcessSettings _scenecapture2d1))) (.FilmContrast (Utilities|Struct|BreakPostProcessSettings (Variables|/Script/Engine.SceneCaptureComponent2D|GetPostProcessSettings _scenecapture2d1))) (.FilmToeAmount (Utilities|Struct|BreakPostProcessSettings (Variables|/Script/Engine.SceneCaptureComponent2D|GetPostProcessSettings _scenecapture2d1))) (.FilmHealAmount (Utilities|Struct|BreakPostProcessSettings (Variables|/Script/Engine.SceneCaptureComponent2D|GetPostProcessSettings _scenecapture2d1))) (.FilmDynamicRange (Utilities|Struct|BreakPostProcessSettings (Variables|/Script/Engine.SceneCaptureComponent2D|GetPostProcessSettings _scenecapture2d1))) (.SceneColorTint (Utilities|Struct|BreakPostProcessSettings (Variables|/Script/Engine.SceneCaptureComponent2D|GetPostProcessSettings _scenecapture2d1))) (.SceneFringeIntensity (Utilities|Struct|BreakPostProcessSettings (Variables|/Script/Engine.SceneCaptureComponent2D|GetPostProcessSettings _scenecapture2d1))) (.SceneFringeSaturation (Utilities|Struct|BreakPostProcessSettings (Variables|/Script/Engine.SceneCaptureComponent2D|GetPostProcessSettings _scenecapture2d1))) (.BloomIntensity (Utilities|Struct|BreakPostProcessSettings (Variables|/Script/Engine.SceneCaptureComponent2D|GetPostProcessSettings _scenecapture2d1))) (.BloomThreshold (Utilities|Struct|BreakPostProcessSettings (Variables|/Script/Engine.SceneCaptureComponent2D|GetPostProcessSettings _scenecapture2d1))) (.Bloom1Size (Utilities|Struct|BreakPostProcessSettings (Variables|/Script/Engine.SceneCaptureComponent2D|GetPostProcessSettings _scenecapture2d1))) (.Bloom2Size (Utilities|Struct|BreakPostProcessSettings (Variables|/Script/Engine.SceneCaptureComponent2D|GetPostProcessSettings _scenecapture2d1))) (.Bloom3Size (Utilities|Struct|BreakPostProcessSettings (Variables|/Script/Engine.SceneCaptureComponent2D|GetPostProcessSettings _scenecapture2d1))) (.Bloom4Size (Utilities|Struct|BreakPostProcessSettings (Variables|/Script/Engine.SceneCaptureComponent2D|GetPostProcessSettings _scenecapture2d1))) (.Bloom5Size (Utilities|Struct|BreakPostProcessSettings (Variables|/Script/Engine.SceneCaptureComponent2D|GetPostProcessSettings _scenecapture2d1))) (.Bloom1Tint (Utilities|Struct|BreakPostProcessSettings (Variables|/Script/Engine.SceneCaptureComponent2D|GetPostProcessSettings _scenecapture2d1))) (.Bloom2Tint (Utilities|Struct|BreakPostProcessSettings (Variables|/Script/Engine.SceneCaptureComponent2D|GetPostProcessSettings _scenecapture2d1))) (.Bloom3Tint (Utilities|Struct|BreakPostProcessSettings (Variables|/Script/Engine.SceneCaptureComponent2D|GetPostProcessSettings _scenecapture2d1))) (.Bloom4Tint (Utilities|Struct|BreakPostProcessSettings (Variables|/Script/Engine.SceneCaptureComponent2D|GetPostProcessSettings _scenecapture2d1))) (.Bloom5Tint (Utilities|Struct|BreakPostProcessSettings (Variables|/Script/Engine.SceneCaptureComponent2D|GetPostProcessSettings _scenecapture2d1))) (.BloomDirtMaskIntensity (Utilities|Struct|BreakPostProcessSettings (Variables|/Script/Engine.SceneCaptureComponent2D|GetPostProcessSettings _scenecapture2d1))) (.BloomDirtMaskTint (Utilities|Struct|BreakPostProcessSettings (Variables|/Script/Engine.SceneCaptureComponent2D|GetPostProcessSettings _scenecapture2d1))) (.BloomDirtMask (Utilities|Struct|BreakPostProcessSettings (Variables|/Script/Engine.SceneCaptureComponent2D|GetPostProcessSettings _scenecapture2d1))) (.LPVIntensity (Utilities|Struct|BreakPostProcessSettings (Variables|/Script/Engine.SceneCaptureComponent2D|GetPostProcessSettings _scenecapture2d1))) (.LPVWarpIntensity (Utilities|Struct|BreakPostProcessSettings (Variables|/Script/Engine.SceneCaptureComponent2D|GetPostProcessSettings _scenecapture2d1))) (.LPVVplInjectionBias (Utilities|Struct|BreakPostProcessSettings (Variables|/Script/Engine.SceneCaptureComponent2D|GetPostProcessSettings _scenecapture2d1))) (.LPVSize (Utilities|Struct|BreakPostProcessSettings (Variables|/Script/Engine.SceneCaptureComponent2D|GetPostProcessSettings _scenecapture2d1))) (.LPVSecondaryOcclusionIntensity (Utilities|Struct|BreakPostProcessSettings (Variables|/Script/Engine.SceneCaptureComponent2D|GetPostProcessSettings _scenecapture2d1))) (.LPVSecondaryBounceIntensity (Utilities|Struct|BreakPostProcessSettings (Variables|/Script/Engine.SceneCaptureComponent2D|GetPostProcessSettings _scenecapture2d1))) (.LPVGeometryVolumeBias (Utilities|Struct|BreakPostProcessSettings (Variables|/Script/Engine.SceneCaptureComponent2D|GetPostProcessSettings _scenecapture2d1))) (.LPVEmissiveInjectionIntensity (Utilities|Struct|BreakPostProcessSettings (Variables|/Script/Engine.SceneCaptureComponent2D|GetPostProcessSettings _scenecapture2d1))) (.LPVTransmissionIntensity (Utilities|Struct|BreakPostProcessSettings (Variables|/Script/Engine.SceneCaptureComponent2D|GetPostProcessSettings _scenecapture2d1))) (.AmbientCubemapTint (Utilities|Struct|BreakPostProcessSettings (Variables|/Script/Engine.SceneCaptureComponent2D|GetPostProcessSettings _scenecapture2d1))) (.AmbientCubemapIntensity (Utilities|Struct|BreakPostProcessSettings (Variables|/Script/Engine.SceneCaptureComponent2D|GetPostProcessSettings _scenecapture2d1))) (.AmbientCubemap (Utilities|Struct|BreakPostProcessSettings (Variables|/Script/Engine.SceneCaptureComponent2D|GetPostProcessSettings _scenecapture2d1))) (.AutoExposureLowPercent (Utilities|Struct|BreakPostProcessSettings (Variables|/Script/Engine.SceneCaptureComponent2D|GetPostProcessSettings _scenecapture2d1))) (.AutoExposureHighPercent (Utilities|Struct|BreakPostProcessSettings (Variables|/Script/Engine.SceneCaptureComponent2D|GetPostProcessSettings _scenecapture2d1))) (.AutoExposureMinBrightness (Utilities|Struct|BreakPostProcessSettings (Variables|/Script/Engine.SceneCaptureComponent2D|GetPostProcessSettings _scenecapture2d1))) (.AutoExposureMaxBrightness (Utilities|Struct|BreakPostProcessSettings (Variables|/Script/Engine.SceneCaptureComponent2D|GetPostProcessSettings _scenecapture2d1))) (.AutoExposureSpeedUp (Utilities|Struct|BreakPostProcessSettings (Variables|/Script/Engine.SceneCaptureComponent2D|GetPostProcessSettings _scenecapture2d1))) (.AutoExposureSpeedDown (Utilities|Struct|BreakPostProcessSettings (Variables|/Script/Engine.SceneCaptureComponent2D|GetPostProcessSettings _scenecapture2d1))) (.AutoExposureBias (Utilities|Struct|BreakPostProcessSettings (Variables|/Script/Engine.SceneCaptureComponent2D|GetPostProcessSettings _scenecapture2d1))) (.HistogramLogMin (Utilities|Struct|BreakPostProcessSettings (Variables|/Script/Engine.SceneCaptureComponent2D|GetPostProcessSettings _scenecapture2d1))) (.HistogramLogMax (Utilities|Struct|BreakPostProcessSettings (Variables|/Script/Engine.SceneCaptureComponent2D|GetPostProcessSettings _scenecapture2d1))) (.LensFlareIntensity (Utilities|Struct|BreakPostProcessSettings (Variables|/Script/Engine.SceneCaptureComponent2D|GetPostProcessSettings _scenecapture2d1))) (.LensFlareTint (Utilities|Struct|BreakPostProcessSettings (Variables|/Script/Engine.SceneCaptureComponent2D|GetPostProcessSettings _scenecapture2d1))) (.LensFlareBokehSize (Utilities|Struct|BreakPostProcessSettings (Variables|/Script/Engine.SceneCaptureComponent2D|GetPostProcessSettings _scenecapture2d1))) (.LensFlareThreshold (Utilities|Struct|BreakPostProcessSettings (Variables|/Script/Engine.SceneCaptureComponent2D|GetPostProcessSettings _scenecapture2d1))) (.LensFlareBokehShape (Utilities|Struct|BreakPostProcessSettings (Variables|/Script/Engine.SceneCaptureComponent2D|GetPostProcessSettings _scenecapture2d1))) (.VignetteIntensity (Utilities|Struct|BreakPostProcessSettings (Variables|/Script/Engine.SceneCaptureComponent2D|GetPostProcessSettings _scenecapture2d1))) (.VignetteColor (Utilities|Struct|BreakPostProcessSettings (Variables|/Script/Engine.SceneCaptureComponent2D|GetPostProcessSettings _scenecapture2d1))) (.GrainJitter (Utilities|Struct|BreakPostProcessSettings (Variables|/Script/Engine.SceneCaptureComponent2D|GetPostProcessSettings _scenecapture2d1))) (.GrainIntensity (Utilities|Struct|BreakPostProcessSettings (Variables|/Script/Engine.SceneCaptureComponent2D|GetPostProcessSettings _scenecapture2d1))) (.AmbientOcclusionIntensity (Utilities|Struct|BreakPostProcessSettings (Variables|/Script/Engine.SceneCaptureComponent2D|GetPostProcessSettings _scenecapture2d1))) (.AmbientOcclusionStaticFraction (Utilities|Struct|BreakPostProcessSettings (Variables|/Script/Engine.SceneCaptureComponent2D|GetPostProcessSettings _scenecapture2d1))) (.AmbientOcclusionRadius (Utilities|Struct|BreakPostProcessSettings (Variables|/Script/Engine.SceneCaptureComponent2D|GetPostProcessSettings _scenecapture2d1))) (.AmbientOcclusionRadiusInWS (Utilities|Struct|BreakPostProcessSettings (Variables|/Script/Engine.SceneCaptureComponent2D|GetPostProcessSettings _scenecapture2d1))) (.AmbientOcclusionFadeDistance (Utilities|Struct|BreakPostProcessSettings (Variables|/Script/Engine.SceneCaptureComponent2D|GetPostProcessSettings _scenecapture2d1))) (.AmbientOcclusionFadeRadius (Utilities|Struct|BreakPostProcessSettings (Variables|/Script/Engine.SceneCaptureComponent2D|GetPostProcessSettings _scenecapture2d1))) (.AmbientOcclusionDistance (Utilities|Struct|BreakPostProcessSettings (Variables|/Script/Engine.SceneCaptureComponent2D|GetPostProcessSettings _scenecapture2d1))) (.AmbientOcclusionPower (Utilities|Struct|BreakPostProcessSettings (Variables|/Script/Engine.SceneCaptureComponent2D|GetPostProcessSettings _scenecapture2d1))) (.AmbientOcclusionBias (Utilities|Struct|BreakPostProcessSettings (Variables|/Script/Engine.SceneCaptureComponent2D|GetPostProcessSettings _scenecapture2d1))) (.AmbientOcclusionQuality (Utilities|Struct|BreakPostProcessSettings (Variables|/Script/Engine.SceneCaptureComponent2D|GetPostProcessSettings _scenecapture2d1))) (.AmbientOcclusionMipBlend (Utilities|Struct|BreakPostProcessSettings (Variables|/Script/Engine.SceneCaptureComponent2D|GetPostProcessSettings _scenecapture2d1))) (.AmbientOcclusionMipScale (Utilities|Struct|BreakPostProcessSettings (Variables|/Script/Engine.SceneCaptureComponent2D|GetPostProcessSettings _scenecapture2d1))) (.AmbientOcclusionMipThreshold (Utilities|Struct|BreakPostProcessSettings (Variables|/Script/Engine.SceneCaptureComponent2D|GetPostProcessSettings _scenecapture2d1))) (.IndirectLightingColor (Utilities|Struct|BreakPostProcessSettings (Variables|/Script/Engine.SceneCaptureComponent2D|GetPostProcessSettings _scenecapture2d1))) (.IndirectLightingIntensity (Utilities|Struct|BreakPostProcessSettings (Variables|/Script/Engine.SceneCaptureComponent2D|GetPostProcessSettings _scenecapture2d1))) (.ColorGradingIntensity (Utilities|Struct|BreakPostProcessSettings (Variables|/Script/Engine.SceneCaptureComponent2D|GetPostProcessSettings _scenecapture2d1))) (.ColorGradingLUT (Utilities|Struct|BreakPostProcessSettings (Variables|/Script/Engine.SceneCaptureComponent2D|GetPostProcessSettings _scenecapture2d1))) (.DepthOfFieldMethod (Utilities|Struct|BreakPostProcessSettings (Variables|/Script/Engine.SceneCaptureComponent2D|GetPostProcessSettings _scenecapture2d1))) (.DepthOfFieldFocalDistance (Utilities|Struct|BreakPostProcessSettings (Variables|/Script/Engine.SceneCaptureComponent2D|GetPostProcessSettings _scenecapture2d1))) (.DepthOfFieldFocalRegion (Utilities|Struct|BreakPostProcessSettings (Variables|/Script/Engine.SceneCaptureComponent2D|GetPostProcessSettings _scenecapture2d1))) (.DepthOfFieldNearTransitionRegion (Utilities|Struct|BreakPostProcessSettings (Variables|/Script/Engine.SceneCaptureComponent2D|GetPostProcessSettings _scenecapture2d1))) (.DepthOfFieldFarTransitionRegion (Utilities|Struct|BreakPostProcessSettings (Variables|/Script/Engine.SceneCaptureComponent2D|GetPostProcessSettings _scenecapture2d1))) (.DepthOfFieldScale (Utilities|Struct|BreakPostProcessSettings (Variables|/Script/Engine.SceneCaptureComponent2D|GetPostProcessSettings _scenecapture2d1))) (.DepthOfFieldMaxBokehSize (Utilities|Struct|BreakPostProcessSettings (Variables|/Script/Engine.SceneCaptureComponent2D|GetPostProcessSettings _scenecapture2d1))) (.DepthOfFieldNearBlurSize (Utilities|Struct|BreakPostProcessSettings (Variables|/Script/Engine.SceneCaptureComponent2D|GetPostProcessSettings _scenecapture2d1))) (.DepthOfFieldFarBlurSize (Utilities|Struct|BreakPostProcessSettings (Variables|/Script/Engine.SceneCaptureComponent2D|GetPostProcessSettings _scenecapture2d1))) (.DepthOfFieldBokehShape (Utilities|Struct|BreakPostProcessSettings (Variables|/Script/Engine.SceneCaptureComponent2D|GetPostProcessSettings _scenecapture2d1))) (.DepthOfFieldOcclusion (Utilities|Struct|BreakPostProcessSettings (Variables|/Script/Engine.SceneCaptureComponent2D|GetPostProcessSettings _scenecapture2d1))) (.DepthOfFieldColorThreshold (Utilities|Struct|BreakPostProcessSettings (Variables|/Script/Engine.SceneCaptureComponent2D|GetPostProcessSettings _scenecapture2d1))) (.DepthOfFieldSizeThreshold (Utilities|Struct|BreakPostProcessSettings (Variables|/Script/Engine.SceneCaptureComponent2D|GetPostProcessSettings _scenecapture2d1))) (.DepthOfFieldSkyFocusDistance (Utilities|Struct|BreakPostProcessSettings (Variables|/Script/Engine.SceneCaptureComponent2D|GetPostProcessSettings _scenecapture2d1))) (.MotionBlurAmount (Utilities|Struct|BreakPostProcessSettings (Variables|/Script/Engine.SceneCaptureComponent2D|GetPostProcessSettings _scenecapture2d1))) (.MotionBlurMax (Utilities|Struct|BreakPostProcessSettings (Variables|/Script/Engine.SceneCaptureComponent2D|GetPostProcessSettings _scenecapture2d1))) (.MotionBlurPerObjectSize (Utilities|Struct|BreakPostProcessSettings (Variables|/Script/Engine.SceneCaptureComponent2D|GetPostProcessSettings _scenecapture2d1))) (.ScreenPercentage (Utilities|Struct|BreakPostProcessSettings (Variables|/Script/Engine.SceneCaptureComponent2D|GetPostProcessSettings _scenecapture2d1))) (.AntiAliasingMethod (Utilities|Struct|BreakPostProcessSettings (Variables|/Script/Engine.SceneCaptureComponent2D|GetPostProcessSettings _scenecapture2d1))) (.ScreenSpaceReflectionIntensity (Utilities|Struct|BreakPostProcessSettings (Variables|/Script/Engine.SceneCaptureComponent2D|GetPostProcessSettings _scenecapture2d1))) (.ScreenSpaceReflectionQuality (Utilities|Struct|BreakPostProcessSettings (Variables|/Script/Engine.SceneCaptureComponent2D|GetPostProcessSettings _scenecapture2d1))) (.ScreenSpaceReflectionMaxRoughness (Utilities|Struct|BreakPostProcessSettings (Variables|/Script/Engine.SceneCaptureComponent2D|GetPostProcessSettings _scenecapture2d1))) (.Blendables (Utilities|Struct|BreakPostProcessSettings (Variables|/Script/Engine.SceneCaptureComponent2D|GetPostProcessSettings _scenecapture2d1)))))
      (if (Variables|Default|GetmemoryTriggered) :!label _label
        (if (!= (Variables|Default|Getcounter) 0)
          (Transformation|SetWorldRotation _camera1 (Class|KismetMathLibrary|MakeRot _pitch (+ _yaw -0.1) _roll) false)
          (Variables|Default|Setcounter (- (Variables|Default|Getcounter) 1)))))
    (else
      (goto _label))))

(fn ConstructionScript)