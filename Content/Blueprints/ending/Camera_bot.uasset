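; Camera_bot is a camera actor in the ending folder that follows the player character at a fixed offset.
; Every Tick, it moves its Camera1 component to player 0's location, shifted along world X and raised in Z, without sweep, smoothing or rotation changes.
; Two unconnected variants remain unused: one follows the capsule at a closer offset, the other moves the whole actor.
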(event EventTick
  (params (DeltaSeconds :type Float%20%28single-precision%29))
  (bind _returnvalue (Game|GetPlayerCharacter 0))
  (bind _returnvalue_2 (Transformation|GetWorldLocation _returnvalue))
  (bind (_x _y _z) (Math|Vector|BreakVector _returnvalue_2))
  (Transformation|SetWorldLocation (Variables|Default|GetCamera1) (Math|Vector|MakeVector (+ _x 4e+02) _y (+ _z 1.5e+02)) false))

(fn ConstructionScript)