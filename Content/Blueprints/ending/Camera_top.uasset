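; Top camera actor for the ending that carries a scene capture and follows the player character at a fixed world offset, updated every tick.
; While IsCheck is set, it steps the capture's post-process film saturation down each frame, then sets SaturationDown once the lower limit is reached.
; Spring-arm attach, rotation and debug-print experiments remain in the graph but never run.
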(event EventTick
  (params (DeltaSeconds :type Float%20%28single-precision%29))
  (bind _returnvalue (Game|GetPlayerCharacter 0))
  (bind _scenecapture2d_top (Variables|Default|GetSceneCapture2D-top))
  (bind _returnvalue_2 (Transformation|GetWorldLocation _returnvalue))
  (bind _postprocesssettings (Variables|/Script/Engine.SceneCaptureComponent2D|GetPostProcessSettings _scenecapture2d_top))
  (bind (_x _y _z) (Math|Vector|BreakVector _returnvalue_2))
  (Transformation|SetActorLocation (Math|Vector|MakeVector (+ _x 4e+02) _y (+ _z 1.5e+02)) false)
  (if (Variables|Default|GetisCheck)
    (if (> (- (Variables|Default|Getsaturation) 0.02) 0.22)
      (Variables|Default|Setsaturation (- (Variables|Default|Getsaturation) 0.02))
      (Utilities|Struct|SetmembersinPostProcessSettings _postprocesssettings false true false false false false false false false false false false false false false false false false false false false false false false false false false false false false false false false false false false false false false false false false false false false false false false false false false false false false false false false false false false false false false false false false false false false false false false false false false false false false false false false false false false false false false false false false false false false false false false false false false false "(R=1.000000,G=1.000000,B=1.000000,A=1.000000)" "(R=1.000000,G=1.000000,B=1.000000,A=1.000000)" 0.5 0.0 (Variables|Default|Getsaturation) "(R=1.000000,G=0.000000,B=0.000000,A=1.000000)" "(R=0.000000,G=1.000000,B=0.000000,A=1.000000)" "(R=0.000000,G=0.000000,B=1.000000,A=1.000000)" 0.03 1.0 0.18 4.0 "(R=1.000000,G=1.000000,B=1.000000,A=1.000000)" 0.0 0.5 1.0 1.0 1.0 4.0 16.0 32.0 1e+02 "(R=0.500000,G=0.500000,B=0.500000,A=1.000000)" "(R=0.500000,G=0.500000,B=0.500000,A=1.000000)" "(R=0.500000,G=0.500000,B=0.500000,A=1.000000)" "(R=0.500000,G=0.500000,B=0.500000,A=1.000000)" "(R=0.500000,G=0.500000,B=0.500000,A=1.000000)" 1.0 "(R=0.500000,G=0.500000,B=0.500000,A=1.000000)" 0 1.0 0.0 0.64 5312.0 0.0 0.0 0.384 1.0 1.0 "(R=1.000000,G=1.000000,B=1.000000,A=1.000000)" 1.0 0 8e+01 98.300003 0.03 2.0 3.0 1.0 0.0 -8.0 4.0 1.0 "(R=1.000000,G=1.000000,B=1.000000,A=1.000000)" 3.0 8.0 0 0.0 "(R=0.000000,G=0.000000,B=0.000000,A=1.000000)" 0.0 0.0 0.5 1.0 4e+01 false 8e+03 5e+03 8e+01 2.0 3.0 5e+01 0.6 1.7 0.01 "(R=1.000000,G=1.000000,B=1.000000,A=1.000000)" 1.0 1.0 0 "DOFM_BokehDOF" 1e+03 0.0 3e+02 5e+02 0.0 15.0 15.0 15.0 0 0.4 1.0 0.08 0.0 0.5 5.0 0.5 1e+02 "AAM_TemporalAA" 1e+02 5e+01 0.6 (.Blendables (Utilities|Struct|BreakPostProcessSettings _postprocesssettings)))
      (else
        (Variables|Default|SetsaturationDown true)))))

(fn ConstructionScript)